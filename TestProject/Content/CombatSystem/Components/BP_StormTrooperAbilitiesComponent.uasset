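; Storm Trooper abilities component, providing an aimed grenade throw and a hit-streak ammo bonus.
; GrenadePredict plays aim montages and predicts the projectile path; Grenade starts a cooldown and spawns the grenade at montage blend-out toward the camera trace.
; GrenadeDamage applies distance-based falloff to hit characters.
; Shooting component events feed hit streaks, the longest setting AmmoToAdd; Dash is empty, its launch logic disconnected.
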(event `self.ReceiveBeginPlay`
  (bind _shootingcomponent (`/Game/CombatSystem/Characters/BP_BaseThirdPersonCharacter.ShootingComponent` (`self.BP_StormTrooperThirdPersonCharacter`)))
  (bind _asbp_storm_trooper_third_person_character (cast `/Game/CombatSystem/Characters/BP_StormTrooperThirdPersonCharacter` (`self.GetOwner`)))
  (set `self.BP_StormTrooperThirdPersonCharacter` _asbp_storm_trooper_third_person_character)
  (`KismetSystemLibrary.DelayUntilNextTick`)
  (add `/Game/CombatSystem/Components/BP_BaseShootingComponent.OnWeaponBeginReload` _shootingcomponent (`|CreateDelegate` :!event `AddHits`))
  (add `/Game/CombatSystem/Components/BP_BaseShootingComponent.OnWeaponAddAmmo` _shootingcomponent (`|CreateDelegate` :!event `GetBiggestHitsInRow`))
  (add `/Game/CombatSystem/Components/BP_BaseShootingComponent.OnAddHitsInRowAmmo` _shootingcomponent (delegate `IncHitsInRow`)))

(event `IncHitsInRow`
  (`/Engine/EditorBlueprintResources/StandardMacros.IncrementFloat` (`self.HitsInRow`)))

(event `Grenade`
  (bind _bp_stormtrooperthirdpersoncharacter (`self.BP_StormTrooperThirdPersonCharacter`))
  (bind _bp_stormtrooperthirdpersoncharacter_2 (`self.BP_StormTrooperThirdPersonCharacter`))
  (bind _bp_stormtrooperthirdpersoncharacter_3 (`self.BP_StormTrooperThirdPersonCharacter`))
  (bind _abp_manny (`/Game/CombatSystem/Characters/BP_BaseThirdPersonCharacter.ABP_Manny` _bp_stormtrooperthirdpersoncharacter_3))
  (bind _shootingcomponent (`/Game/CombatSystem/Characters/BP_BaseThirdPersonCharacter.ShootingComponent` _bp_stormtrooperthirdpersoncharacter))
  (bind _returnvalue (`SceneComponent.GetSocketLocation` (`Character.Mesh` _bp_stormtrooperthirdpersoncharacter_2) "hand_l"))
  ;[0.006141 1 0] StormTrooper Grenade / Second Ability
  (if (`GameplayTagAssetInterface.HasMatchingGameplayTag` (`/Game/CombatSystem/Characters/BP_BaseThirdPersonCharacter.AbilitySystemComponent` _bp_stormtrooperthirdpersoncharacter_3) (struct :`TagName` "PlayerState.IsAiming"))
    (set `/Game/Characters/Mannequins/Animations/ABP_Manny.IsUpperBody` true _abp_manny)
    (`|PlayMontage` (`Character.Mesh` _bp_stormtrooperthirdpersoncharacter_3) "/Game/CombatSystem/Animations/AM_MM_Rifle_GrenadeToss.AM_MM_Rifle_GrenadeToss"
      (:`then`
        (set `self.DoesSecondStormTrooperAbilityCooldownEnd` false)
        (`KismetSystemLibrary.Delay` 1.0)
        (set `self.DoesSecondStormTrooperAbilityCooldownEnd` true))
      (:`OnCompleted`
        (set `/Game/CombatSystem/Components/BP_BaseShootingComponent.IsGrenadeThrow` false _shootingcomponent)
        (`/Game/CombatSystem/Components/BP_BaseShootingComponent.AttachWeapon` _shootingcomponent (`/Game/CombatSystem/Characters/BP_BaseThirdPersonCharacter.CurrentWeaponBlueprint` _bp_stormtrooperthirdpersoncharacter)))
      (:`OnBlendOut`
        (set `/Game/Characters/Mannequins/Animations/ABP_Manny.IsUpperBody` false _abp_manny)
        (bind _outhit (`/Game/CombatSystem/Components/BP_BaseShootingComponent.GetCameraForwardTraceHit` _shootingcomponent))
        (bind (_bblockinghit _binitialoverlap _time _distance _location) (`GameplayStatics.BreakHitResult` _outhit))
        (bind _returnvalue_2 (`|SpawnActorFromClass` "/Game/CombatSystem/Weapons/Grenade/BP_Grenade.BP_Grenade_C" (`KismetMathLibrary.MakeTransform` _returnvalue (`KismetMathLibrary.SelectRotator` (`KismetMathLibrary.Conv_VectorToRotator` (`KismetMathLibrary.GetDirectionUnitVector` _returnvalue _location)) (`Actor.K2_GetActorRotation` (`GameplayStatics.GetPlayerCameraManager` 0)) _bblockinghit)) "AlwaysSpawn" "MultiplyWithRoot" _bp_stormtrooperthirdpersoncharacter_2 _bp_stormtrooperthirdpersoncharacter_2))
        (set `self.BP_Grenade` _returnvalue_2)))))

(event `GrenadePredict`
  (bind _bp_stormtrooperthirdpersoncharacter (`self.BP_StormTrooperThirdPersonCharacter`))
  (bind _bp_stormtrooperthirdpersoncharacter_2 (`self.BP_StormTrooperThirdPersonCharacter`))
  (bind _bp_stormtrooperthirdpersoncharacter_3 (`self.BP_StormTrooperThirdPersonCharacter`))
  (bind _shootingcomponent (`/Game/CombatSystem/Characters/BP_BaseThirdPersonCharacter.ShootingComponent` _bp_stormtrooperthirdpersoncharacter))
  (bind _mesh (`Character.Mesh` _bp_stormtrooperthirdpersoncharacter_2))
  ;[0.006141 1 0] StormTrooper Grenade / Second Ability
  (set `/Game/CombatSystem/Components/BP_BaseShootingComponent.IsGrenadeThrow` true _shootingcomponent)
  (`/Game/CombatSystem/Components/BP_BaseShootingComponent.AttachSecondWeapon` _shootingcomponent (`/Game/CombatSystem/Characters/BP_BaseThirdPersonCharacter.CurrentWeaponBlueprint` _bp_stormtrooperthirdpersoncharacter))
  (if (and (`self.DoesSecondStormTrooperAbilityCooldownEnd`) (`GameplayTagAssetInterface.HasMatchingGameplayTag` (`/Game/CombatSystem/Characters/BP_BaseThirdPersonCharacter.AbilitySystemComponent` _bp_stormtrooperthirdpersoncharacter) (struct :`TagName` "PlayerState.IsAiming")))
    (set `/Game/Characters/Mannequins/Animations/ABP_Manny.IsUpperBody` true (`/Game/CombatSystem/Characters/BP_BaseThirdPersonCharacter.ABP_Manny` _bp_stormtrooperthirdpersoncharacter_2))
    (`|PlayMontage` _mesh "/Game/CombatSystem/Animations/AM_MM_Rifle_GrenadeToss.AM_MM_Rifle_GrenadeToss" 1.0 0.0 "GrenadeAim"
      (:`OnCompleted`
        (`|PlayMontage` _mesh "/Game/CombatSystem/Animations/AM_MM_Rifle_GrenadeToss_1.AM_MM_Rifle_GrenadeToss_1"
          (:`then`
            (`GameplayStatics.Blueprint_PredictProjectilePath_Advanced` (make `PredictProjectilePathParams` :`StartLocation` (`SceneComponent.GetSocketLocation` (`Character.Mesh` (`self.BP_StormTrooperThirdPersonCharacter`)) "hand_l") :`LaunchVelocity` (* (`Actor.GetActorForwardVector` (`GameplayStatics.GetPlayerCameraManager` 0)) (`self.InitialGrenadeSpeed`)) :`bTraceWithCollision` true :`ProjectileRadius` 16.0 :`ActorsToIgnore` (`|MakeArray` _bp_stormtrooperthirdpersoncharacter_3 (`/Game/CombatSystem/Characters/BP_BaseThirdPersonCharacter.CurrentWeaponBlueprint` _bp_stormtrooperthirdpersoncharacter_3) :!type "Actor Object Reference") :`DrawDebugType` "ForOneFrame"))))))))

(event `Dash`
  ;[0.006141 1 0] StormTrooper Dash / Movement Ability
)

(fn `AddHits`
  (locals (LocalDefaultValue :type "Float (double-precision)"))
  (`BlueprintMapLibrary.Map_Add` (`self.SeriesHitsInRowValues`) (`self.HitsInRowSeries`) (make `/Game/CombatSystem/Structures/S_SeriesHitsInRowValues` (`self.HitsInRow`)))
  (set `self.HitsInRow` (`local.LocalDefaultValue`))
  (`/Engine/EditorBlueprintResources/StandardMacros.IncrementInt` (`self.HitsInRowSeries`)))

(fn `GetBiggestHitsInRow`
  (locals (LocalDefaultValue :type "Float (double-precision)") (LocalLastHitsValue :type "Float (double-precision)"))
  (set `local.LocalLastHitsValue` (`local.LocalDefaultValue`))
  (bind _keys (`BlueprintMapLibrary.Map_Keys` (`self.SeriesHitsInRowValues`)))
  (for _array_element _keys
    (bind _value (`BlueprintMapLibrary.Map_Find` (`self.SeriesHitsInRowValues`) _array_element))
    (if (> (break `/Game/CombatSystem/Structures/S_SeriesHitsInRowValues` _value) (`local.LocalLastHitsValue`))
      (set `local.LocalLastHitsValue` (break `/Game/CombatSystem/Structures/S_SeriesHitsInRowValues` _value))))
  (`BlueprintMapLibrary.Map_Clear` (`self.SeriesHitsInRowValues`))
  (set `self.HitsInRowSeries` 0)
  (set `/Game/CombatSystem/Components/BP_BaseShootingComponent.AmmoToAdd` (`local.LocalLastHitsValue`) (`/Game/CombatSystem/Characters/BP_BaseThirdPersonCharacter.ShootingComponent` (`self.BP_StormTrooperThirdPersonCharacter`)))
  (return))

(fn `GrenadeDamage`
  (params (NewParam :type "Array of HitResult Structure"))
  (locals (LocalLastHitActor :type "Actor Object Reference") (LocalDistanceMultiplier :type "Float (double-precision)" :default 100.0) (LocalMinGrenadeDamage :type "Float (double-precision)" :default 15.0) (LocalMaxGrenadeDamage :type "Float (double-precision)" :default 125.0))
  (bind _damagesphereradius (`/Game/CombatSystem/Weapons/Grenade/BP_Grenade.DamageSphereRadius` (`self.BP_Grenade`)))
  (for _array_element NewParam
    (bind (_bblockinghit _binitialoverlap _time _distance _location _impactpoint _normal _impactnormal _physmat _hitactor) (`GameplayStatics.BreakHitResult` _array_element))
    (cast `/Game/CombatSystem/Characters/BP_BaseThirdPersonCharacter` _hitactor)
    (if (!= _hitactor (`local.LocalLastHitActor`))
      (`GameplayStatics.ApplyDamage` _hitactor (`KismetMathLibrary.FClamp` (- (`local.LocalMaxGrenadeDamage`) (* (/ (`KismetMathLibrary.FClamp` (`KismetMathLibrary.VSize` (- (`Actor.K2_GetActorLocation` (`self.BP_Grenade`)) (`Actor.K2_GetActorLocation` _hitactor))) 0.0 _damagesphereradius) _damagesphereradius) (`local.LocalDistanceMultiplier`))) (`local.LocalMinGrenadeDamage`) (`local.LocalMaxGrenadeDamage`)))
      (set `local.LocalLastHitActor` _hitactor))))