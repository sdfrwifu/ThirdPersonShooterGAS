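; Component on the Engineer character that runs its abilities: a timed-cooldown shotgun spread modifier, drone spawning and a movement boost.
; It binds to ShootingComponent fire and blast-loop events, counting shots to end the spread ability.
; The movement ability temporarily raises walk speed and jump velocity.
; Drone aura functions apply and revert multiplied speed and added blast amount.
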(event `self.ReceiveBeginPlay`
  (bind _asbp_engineer_third_person_character (cast `/Game/CombatSystem/Characters/BP_EngineerThirdPersonCharacter` (`self.GetOwner`)))
  (set `self.BP_EngineerThirdPersonCharacter` _asbp_engineer_third_person_character)
  (`KismetSystemLibrary.DelayUntilNextTick`)
  (bind _shootingcomponent (`/Game/CombatSystem/Characters/BP_BaseThirdPersonCharacter.ShootingComponent` _asbp_engineer_third_person_character))
  (add `/Game/CombatSystem/Components/BP_BaseShootingComponent.OnShotgunFire` _shootingcomponent (`|CreateDelegate` :!event `OnShotgunFire`))
  (add `/Game/CombatSystem/Components/BP_BaseShootingComponent.OnBlastLoopCompleted` _shootingcomponent (delegate `OnBlastLoopCompleted`)))

(event `OnBlastLoopCompleted`
  (if (`self.IsFirstEngineerAbility`)
    (`/Engine/EditorBlueprintResources/StandardMacros.IncrementInt` (`self.AmountOfShotsAbility`))))

(event `EngineerFirstAbility`
  ;[0.006141 1 0] First Engineer Ability
  (set `self.DoesFirstEngineerAbilityCooldownEnd` false)
  (set `self.IsFirstEngineerAbility` true)
  (`KismetSystemLibrary.Delay` 20.0)
  (set `self.DoesFirstEngineerAbilityCooldownEnd` true))

(event `SpawnDrone`
  (params (DroneOwner :type "Actor Object Reference"))
  ;[0.006141 1 0] Second Ability / Drone
  (`|SpawnActorFromClass` "/Game/CombatSystem/Drone/DronePawn.DronePawn_C" (`KismetMathLibrary.MakeTransform` (+ (* (`Actor.GetActorForwardVector` DroneOwner) 300.0) (`Actor.K2_GetActorLocation` DroneOwner)) (`Actor.K2_GetActorRotation` DroneOwner)) "AlwaysSpawn" "MultiplyWithRoot" DroneOwner DroneOwner))

(event `EngineerMovementAbility`
  (bind _bp_engineerthirdpersoncharacter (`self.BP_EngineerThirdPersonCharacter`))
  (bind _charactermovement (`Character.CharacterMovement` _bp_engineerthirdpersoncharacter))
  (`|ExecutionSequence`
    (:`then_0`
      (set `self.DoesEngineerMovementAbilityCooldownEnd` false)
      (`KismetSystemLibrary.Delay` 30.0)
      (set `self.DoesEngineerMovementAbilityCooldownEnd` true))
    (:`then_1`
      (set `CharacterMovementComponent.MaxWalkSpeed` (`self.MaxAbilityWalkSpeed`) _charactermovement)
      (bind _output_get (set `CharacterMovementComponent.JumpZVelocity` (* (`CharacterMovementComponent.JumpZVelocity` _charactermovement) (`self.AbilityJumpMultiplier`)) _charactermovement))
      (`KismetSystemLibrary.Delay` 10.0)
      (set `CharacterMovementComponent.MaxWalkSpeed` (`/Game/CombatSystem/Components/BP_BaseShootingComponent.MaxDefaultCharacterSpeed` (`/Game/CombatSystem/Characters/BP_BaseThirdPersonCharacter.ShootingComponent` _bp_engineerthirdpersoncharacter)) _charactermovement)
      (set `CharacterMovementComponent.JumpZVelocity` (/ _output_get (`self.AbilityJumpMultiplier`)) _charactermovement))))

(fn `DecreaseCharacterAuraStats`
  (bind _shootingcomponent (`/Game/CombatSystem/Characters/BP_BaseThirdPersonCharacter.ShootingComponent` (`self.BP_EngineerThirdPersonCharacter`)))
  (set `self.IsInDroneAura` false)
  (bind _asbp_engineer_third_person_character (cast `/Game/CombatSystem/Characters/BP_EngineerThirdPersonCharacter` (`self.GetOwner`)))
  (bind _charactermovement (`Character.CharacterMovement` _asbp_engineer_third_person_character))
  (set `CharacterMovementComponent.MaxWalkSpeed` (/ (`MovementComponent.GetMaxSpeed` _charactermovement) (`self.SpeedMultiplierInDroneAura`)) _charactermovement)
  (set `/Game/CombatSystem/Components/BP_BaseShootingComponent.EnginnerBlastAmount` (- (`/Game/CombatSystem/Components/BP_BaseShootingComponent.EnginnerBlastAmount` _shootingcomponent) (`self.BlastAmountInreaseInDroneAura`)) _shootingcomponent))

(fn `IncreaseCharacterAuraStats`
  (bind _shootingcomponent (`/Game/CombatSystem/Characters/BP_BaseThirdPersonCharacter.ShootingComponent` (`self.BP_EngineerThirdPersonCharacter`)))
  (set `self.IsInDroneAura` true)
  (bind _asbp_engineer_third_person_character (cast `/Game/CombatSystem/Characters/BP_EngineerThirdPersonCharacter` (`self.GetOwner`)))
  (bind _charactermovement (`Character.CharacterMovement` _asbp_engineer_third_person_character))
  (set `CharacterMovementComponent.MaxWalkSpeed` (* (`MovementComponent.GetMaxSpeed` _charactermovement) (`self.SpeedMultiplierInDroneAura`)) _charactermovement)
  (set `/Game/CombatSystem/Components/BP_BaseShootingComponent.EnginnerBlastAmount` (+ (`/Game/CombatSystem/Components/BP_BaseShootingComponent.EnginnerBlastAmount` _shootingcomponent) (`self.BlastAmountInreaseInDroneAura`)) _shootingcomponent))

(fn `OnShotgunFire`
  (locals (LocalMaxAmountOfShotsAbility :type Integer :default 5) (LocalAbilitySpreadMultiplier :type "Float (double-precision)" :default 0.5))
  (if (>= (`self.AmountOfShotsAbility`) (`local.LocalMaxAmountOfShotsAbility`))
    (set `self.IsFirstEngineerAbility` false)
    (set `self.AmountOfShotsAbility` 0)
    (elif (`self.IsFirstEngineerAbility`)
      (set `/Game/CombatSystem/Components/BP_BaseShootingComponent.EngineerSpreadMultiplier` (`local.LocalAbilitySpreadMultiplier`) (`/Game/CombatSystem/Characters/BP_BaseThirdPersonCharacter.ShootingComponent` (`self.BP_EngineerThirdPersonCharacter`))))))