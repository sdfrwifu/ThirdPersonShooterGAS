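; Projectile Blueprint for a self-guiding bullet in the combat system that steers toward an automatically chosen target.
; HomingProjectile has TargetingComponent gather targets and pick the best, then sets that target's Chest as the ProjectileMovement homing target.
; A looping timer runs HomingSpeedChange to step an alpha that lerps homing acceleration from minimum to maximum.
; The timer clears when the alpha exactly equals its end value.
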(event `self.ReceiveBeginPlay`
  (`parent.ReceiveBeginPlay`))

(event `HomingProjectile`
  (bind _targetingcomponent (`self.TargetingComponent`))
  (bind _projectilemovement (`self.ProjectileMovement`))
  (bind _currenttarget (`/Game/CombatSystem/Components/BP_TargetingComponent.CurrentTarget` _targetingcomponent))
  ;[0 0.08041 1] убираем в пулю
  ;;[0.006141 1 0] Auto Homing
  (`/Game/CombatSystem/Components/BP_TargetingComponent.AddTargets` _targetingcomponent)
  (`/Game/CombatSystem/Components/BP_TargetingComponent.FindBestTarget` _targetingcomponent)
  (`/Engine/EditorBlueprintResources/StandardMacros.IsValid` _currenttarget
    (:`Is Valid`
      (set `ProjectileMovementComponent.HomingTargetComponent` (`/Game/CombatSystem/Characters/BP_BaseThirdPersonCharacter.Chest` _currenttarget) _projectilemovement)
      ;[0.5208 0.004521 0] Мб это компонент прожектайла умеет делать?
      (set `ProjectileMovementComponent.bIsHomingProjectile` true _projectilemovement)
      (bind _returnvalue (`KismetSystemLibrary.K2_SetTimerDelegate` (delegate `HomingSpeed`) (`self.HomingLerpTickTimeRate`) true))
      (set `self.HomingTimer` _returnvalue))))

(event `HomingSpeed`
  ;[0.5208 0.004521 0] Мб это компонент прожектайла умеет делать?
  (`self.HomingSpeedChange`))

(fn `HomingSpeedChange`
  (locals (LocalMinHomingAlpha :type "Float (double-precision)") (LocalMaxHomingAlpha :type "Float (double-precision)" :default 1.0) (LocalMinHomingAccelerationMagnitude :type "Float (double-precision)" :default 1000.0) (LocalMaxHomingAccelerationMagnitude :type "Float (double-precision)" :default 100000.0) (LocalHomingLerpEnd :type "Float (double-precision)" :default 1.0) (LocalHomingLerpChangeRate :type "Float (double-precision)" :default 0.1))
  (`/Engine/EditorBlueprintResources/StandardMacros.IsValid` self
    (:`Is Valid`
      (bind _output_get (set `self.HomingAlpha` (+ (`KismetMathLibrary.FClamp` (`self.HomingAlpha`) (`local.LocalMinHomingAlpha`) (`local.LocalMaxHomingAlpha`)) (`local.LocalHomingLerpChangeRate`))))
      (`/Engine/EditorBlueprintResources/StandardMacros.IsValid` self
        (:`Is Valid`
          (set `ProjectileMovementComponent.HomingAccelerationMagnitude` (`KismetMathLibrary.Lerp` (`local.LocalMinHomingAccelerationMagnitude`) (`local.LocalMaxHomingAccelerationMagnitude`) _output_get) (`self.ProjectileMovement`))
          (if (== (`self.HomingAlpha`) (`local.LocalHomingLerpEnd`))
            (`KismetSystemLibrary.K2_ClearAndInvalidateTimerHandle` (`self.HomingTimer`))))))
    (:`Is Not Valid`
      (`KismetSystemLibrary.K2_ClearAndInvalidateTimerHandle` (`self.HomingTimer`)))))

(fn `UserConstructionScript`
  (`parent.UserConstructionScript`))