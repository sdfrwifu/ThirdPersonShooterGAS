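; Sniper's second Gameplay Ability, which equips the current weapon: attaches it, sets ammo, plays the rifle equip montage and applies walk speed.
; On activation it resets FOV and eases the camera boom offset back to default on a looping timer.
; It binds to ShootingComponent events for headshots and aiming changes, with helpers for head damage multiplier, pistol-dependent speed and tag-driven scope FOV and HUD.
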(event `self.K2_ActivateAbility`
  (bind _sniperthirdpersoncharacter (`self.SniperThirdPersonCharacter`))
  (bind _sniperthirdpersoncharacter_2 (`self.SniperThirdPersonCharacter`))
  (bind _shootingcomponent (`/Game/CombatSystem/Characters/BP_BaseThirdPersonCharacter.ShootingComponent` _sniperthirdpersoncharacter_2))
  (`self.K2_CommitAbility`)
  (bind _asbp_sniper_third_person_character (cast `/Game/CombatSystem/Characters/BP_SniperThirdPersonCharacter` (`self.GetAvatarActorFromActorInfo`)))
  (bind _output_get (set `self.SniperThirdPersonCharacter` _asbp_sniper_third_person_character))
  (`CameraComponent.SetFieldOfView` (`/Game/CombatSystem/Characters/BP_BaseThirdPersonCharacter.ThirdPersonCamera` _output_get) (`/Game/CombatSystem/Characters/BP_BaseThirdPersonCharacter.DefaultFOV` _output_get))
  (set `self.CurrentSpringArmOffset` (`SpringArmComponent.SocketOffset` (`/Game/CombatSystem/Characters/BP_BaseThirdPersonCharacter.CameraBoom` (`self.SniperThirdPersonCharacter`))))
  (bind _returnvalue (`KismetSystemLibrary.K2_SetTimerDelegate` (delegate `ReturnCamera`) (`self.AimingLerpTickTimeRate`) true))
  (set `self.ReturnCameraTimer` _returnvalue)
  (`/Game/CombatSystem/Components/BP_BaseShootingComponent.NotAimingSettings` _shootingcomponent)
  (`/Game/CombatSystem/Components/BP_BaseShootingComponent.AttachWeapon` _shootingcomponent (`/Game/CombatSystem/Characters/BP_BaseThirdPersonCharacter.CurrentWeaponBlueprint` _sniperthirdpersoncharacter_2))
  (`/Game/CombatSystem/Components/BP_BaseShootingComponent.SetAmmo` _shootingcomponent)
  (`self.BindEvents`)
  (`self.SetNotAimingSettings`)
  (set `CharacterMovementComponent.MaxWalkSpeed` (`/Game/CombatSystem/Components/BP_BaseShootingComponent.CurrentMaxCharacterSpeed` (`/Game/CombatSystem/Characters/BP_BaseThirdPersonCharacter.ShootingComponent` _sniperthirdpersoncharacter)) (`Character.CharacterMovement` _sniperthirdpersoncharacter))
  (`|PlayMontage` (`Character.Mesh` (`self.SniperThirdPersonCharacter`)) "/Game/CombatSystem/Animations/AM_MM_Rifle_Equip.AM_MM_Rifle_Equip"))

(event `ReturnCamera`
  (`self.ReturnCameraChange`))

(fn `BindEvents`
  (bind _shootingcomponent (`/Game/CombatSystem/Characters/BP_BaseThirdPersonCharacter.ShootingComponent` (`self.SniperThirdPersonCharacter`)))
  (add `/Game/CombatSystem/Components/BP_BaseShootingComponent.OnHeadHit` _shootingcomponent (`|CreateDelegate` :!event `SetHeadDamageMultiplier`))
  (add `/Game/CombatSystem/Components/BP_BaseShootingComponent.OnNotAimingSettings` _shootingcomponent (`|CreateDelegate` :!event `SetNotAimingSettings`))
  (add `/Game/CombatSystem/Components/BP_BaseShootingComponent.OnAimingSetFOV` _shootingcomponent (`|CreateDelegate` :!event `SetAimingFOV`)))

(fn `ReturnCameraChange`
  (locals (LocalSpringArmChangeRate :type "Float (double-precision)" :default 0.025) (LocalDefaultSpringArmOffset :type "Vector Structure") (LocalLerpEndAlpha :type "Float (double-precision)" :default 1.0))
  (bind _output_get (set `self.SpringArmAlpha` (+ (`self.SpringArmAlpha`) (`local.LocalSpringArmChangeRate`))))
  (set `SpringArmComponent.SocketOffset` (`KismetMathLibrary.VLerp` (`self.CurrentSpringArmOffset`) (`local.LocalDefaultSpringArmOffset`) _output_get) (`/Game/CombatSystem/Characters/BP_BaseThirdPersonCharacter.CameraBoom` (`self.SniperThirdPersonCharacter`)))
  (if (>= (`self.SpringArmAlpha`) (`local.LocalLerpEndAlpha`))
    (`KismetSystemLibrary.K2_ClearAndInvalidateTimerHandle` (`self.ReturnCameraTimer`))))

(fn `SetAimingFOV`
  (locals (LocalScopingFOV :type "Float (single-precision)" :default 27.0))
  (bind _sniperthirdpersoncharacter (`self.SniperThirdPersonCharacter`))
  (bind _hud (`/Game/CombatSystem/Characters/BP_BaseThirdPersonCharacter.HUD` _sniperthirdpersoncharacter))
  (bind _aimimage (`/Game/CombatSystem/Hud/CharacterHud.AimImage` _hud))
  (if (`GameplayTagAssetInterface.HasMatchingGameplayTag` (`/Game/CombatSystem/Characters/BP_BaseThirdPersonCharacter.AbilitySystemComponent` (`self.SniperThirdPersonCharacter`)) (struct :`TagName` "PlayerState.IsScoping"))
    (`CameraComponent.SetFieldOfView` (`/Game/CombatSystem/Characters/BP_BaseThirdPersonCharacter.ThirdPersonCamera` _sniperthirdpersoncharacter) (`local.LocalScopingFOV`))
    (`Widget.SetVisibility` _aimimage "Hidden")
    (`Widget.SetVisibility` (`/Game/CombatSystem/Hud/CharacterHud.ScopeImage` _hud) "Visible")
    (else
      (`Widget.SetVisibility` (`/Game/CombatSystem/Hud/CharacterHud.ScopeImage` _hud) "Hidden")
      (`Widget.SetVisibility` _aimimage "Visible"))))

(fn `SetHeadDamageMultiplier`
  (locals (LocalHeadDamageMultiplier :type "Float (double-precision)" :default 1.5))
  (set `/Game/CombatSystem/Components/BP_BaseShootingComponent.DamageMultiplier` (`local.LocalHeadDamageMultiplier`) (`/Game/CombatSystem/Characters/BP_BaseThirdPersonCharacter.ShootingComponent` (`self.SniperThirdPersonCharacter`))))

(fn `SetNotAimingSettings`
  (bind _sniperthirdpersoncharacter (`self.SniperThirdPersonCharacter`))
  (bind _sniperthirdpersoncharacter_2 (`self.SniperThirdPersonCharacter`))
  (set `/Game/CombatSystem/Components/BP_BaseShootingComponent.CurrentMaxCharacterSpeed` (`KismetMathLibrary.SelectFloat` (`self.MaxPistolCharacterSpeed`) (`self.MaxDefaultCharacterSpeed`) (`/Game/CombatSystem/Characters/BP_SniperThirdPersonCharacter.IsCurrentWeaponPistol` _sniperthirdpersoncharacter)) (`/Game/CombatSystem/Characters/BP_BaseThirdPersonCharacter.ShootingComponent` _sniperthirdpersoncharacter))
  (if (`GameplayTagAssetInterface.HasMatchingGameplayTag` (`/Game/CombatSystem/Characters/BP_BaseThirdPersonCharacter.AbilitySystemComponent` (`self.SniperThirdPersonCharacter`)) (struct :`TagName` "PlayerState.IsScoping"))
    (`CameraComponent.SetFieldOfView` (`/Game/CombatSystem/Characters/BP_BaseThirdPersonCharacter.ThirdPersonCamera` _sniperthirdpersoncharacter_2) (`/Game/CombatSystem/Characters/BP_BaseThirdPersonCharacter.DefaultFOV` _sniperthirdpersoncharacter_2))))