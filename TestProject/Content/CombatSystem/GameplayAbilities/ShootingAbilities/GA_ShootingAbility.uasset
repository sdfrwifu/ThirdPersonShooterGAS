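; Gameplay ability that fires one hitscan shot from the avatar's current weapon while the player is aiming and has ammo.
; It plays weapon sound and FX, subtracts ammo, then uses a camera trace to find the aim point.
; A multi-line trace runs from the muzzle past that point, or to the camera trace end, and feeds its hits to TraceDamage.
; Failing the aim or ammo check clears the full-auto timer.
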(event `self.K2_ActivateAbility`
  (bind _returnvalue (`SceneComponent.K2_GetComponentLocation` (`/Game/CombatSystem/Weapons/BP_BaseWeapon.Muzzle` (`self.BaseWeaponBlueprint`))))
  (bind _asbp_base_third_person_character (cast `/Game/CombatSystem/Characters/BP_BaseThirdPersonCharacter` (`self.GetAvatarActorFromActorInfo`)))
  (set `self.BaseWeaponBlueprint` (`/Game/CombatSystem/Characters/BP_BaseThirdPersonCharacter.CurrentWeaponBlueprint` _asbp_base_third_person_character))
  ;[0.03253 0 1] Убираем в функцию тк реюзаем
  (if (and (`GameplayTagAssetInterface.HasAllMatchingGameplayTags` (`/Game/CombatSystem/Characters/BP_BaseThirdPersonCharacter.AbilitySystemComponent` _asbp_base_third_person_character) (`BlueprintGameplayTagLibrary.MakeLiteralGameplayTagContainer` (struct :`GameplayTags` (struct :`(TagName` "PlayerState.IsAiming") :`(TagName` "PlayerState.IsFireButtonPressed") :`(TagName` "PlayerState.IsReloadCompleted"))))) (> (`self.CurrentAmountOfAmmo`) 0.0))
    (`/Game/CombatSystem/Weapons/BP_BaseWeapon.SpawnSoundAndFX` (`self.BaseWeaponBlueprint`))
    (`self.AmmoSubtract`)
    (bind _outhit (`self.GetCameraTraceHit`))
    (bind (_bblockinghit _binitialoverlap _time _distance _location _impactpoint _normal _impactnormal _physmat _hitactor _hitcomponent _hitbonename _bonename _hititem _elementindex _faceindex _tracestart _traceend) (`GameplayStatics.BreakHitResult` _outhit))
    (bind _returnvalue_2 (- _location _returnvalue))
    (bind _outhits (`KismetSystemLibrary.LineTraceMulti` :`Start` _returnvalue :`End` (`KismetMathLibrary.SelectVector` (+ (* (/ _returnvalue_2 (`KismetMathLibrary.VSize` _returnvalue_2)) (`self.ShootingDistanceMultiplayer`)) _location) _traceend _bblockinghit) :`TraceChannel` "TraceTypeQuery1" :`DrawDebugType` "ForDuration" :`bIgnoreSelf` false))
    (`self.TraceDamage` _outhits)
    (else
      (`KismetSystemLibrary.K2_ClearAndInvalidateTimerHandle` (`self.FullAutoTimer`)))))