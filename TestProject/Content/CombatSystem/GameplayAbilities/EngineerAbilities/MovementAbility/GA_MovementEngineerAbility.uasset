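; Gameplay ability for the Engineer's movement skill, temporarily boosting the avatar's walk speed and jump.
; On activation it commits, force-applies cooldown, then sets MaxWalkSpeed and multiplies JumpZVelocity on the character movement component directly.
; After a fixed ten-second Delay it restores speed from the ShootingComponent's default, divides the jump multiplier back out and ends the ability.
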(event `self.K2_ActivateAbility`
  (`self.K2_CommitAbility`)
  (`self.K2_CommitAbilityCooldown` false true)
  (bind _asbp_base_third_person_character (cast `/Game/CombatSystem/Characters/BP_BaseThirdPersonCharacter` (`self.GetAvatarActorFromActorInfo`)))
  (bind _charactermovement (`Character.CharacterMovement` _asbp_base_third_person_character))
  (set `CharacterMovementComponent.MaxWalkSpeed` (`self.MaxAbilityWalkSpeed`) _charactermovement)
  (bind _output_get (set `CharacterMovementComponent.JumpZVelocity` (* (`CharacterMovementComponent.JumpZVelocity` _charactermovement) (`self.AbilityJumpMultiplier`)) _charactermovement))
  (`KismetSystemLibrary.Delay` 10.0)
  (set `CharacterMovementComponent.MaxWalkSpeed` (`/Game/CombatSystem/Components/BP_BaseShootingComponent.MaxDefaultCharacterSpeed` (`/Game/CombatSystem/Characters/BP_BaseThirdPersonCharacter.ShootingComponent` _asbp_base_third_person_character)) _charactermovement)
  (set `CharacterMovementComponent.JumpZVelocity` (/ _output_get (`self.AbilityJumpMultiplier`)) _charactermovement)
  (`self.K2_EndAbility`))