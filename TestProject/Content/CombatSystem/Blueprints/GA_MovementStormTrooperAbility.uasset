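; GA_MovementStormTrooperAbility is a gameplay ability that makes the storm trooper dash along its current movement.
; On activation it swaps the owner's upper-body state effect for full-body and plays a forward dash montage.
; It launches the character using horizontal velocity scaled by a dash multiplier, then forces the cooldown.
; When the montage completes, blends out or is interrupted or cancelled, it restores the upper-body state and ends.
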(event `self.K2_ActivateAbility`
  (`self.K2_CommitAbility`)
  (`self.BP_ApplyGameplayEffectToOwner` "/Game/CombatSystem/Blueprints/GE_IsFullBody.GE_IsFullBody_C")
  (`self.BP_RemoveGameplayEffectFromOwnerWithGrantedTags` (struct :`GameplayTags` (struct :`(TagName` "PlayerState.IsUpperBody"))))
  (`AbilityTask_PlayMontageAndWait.CreatePlayMontageAndWaitProxy` "None" "/Game/CombatSystem/Animations/AM_MM_Dash_Forward.AM_MM_Dash_Forward"
    (:`then`
      (bind _asbp_base_third_person_character (cast `/Game/CombatSystem/Characters/BP_BaseThirdPersonCharacter` (`self.GetAvatarActorFromActorInfo`)))
      (bind (_returnvalue_x _returnvalue_y) (`KismetMathLibrary.BreakVector` (* (`Actor.GetVelocity` _asbp_base_third_person_character) (`self.DashVelocityMultiplier`))))
      (`Character.LaunchCharacter` _asbp_base_third_person_character (`KismetMathLibrary.MakeVector` _returnvalue_x _returnvalue_y) false false)
      (`self.K2_CommitAbilityCooldown` false true))
    (:`OnCompleted`
      (`self.BP_ApplyGameplayEffectToOwner` "/Game/CombatSystem/Blueprints/GE_IsUpperBody.GE_IsUpperBody_C" :!label _label)
      (`self.BP_RemoveGameplayEffectFromOwnerWithGrantedTags` (struct :`GameplayTags` (struct :`(TagName` "PlayerState.IsFullBody"))))
      (`self.K2_EndAbility`))
    (:`OnBlendOut`
      (goto _label))
    (:`OnInterrupted`
      (goto _label))
    (:`OnCancelled`
      (goto _label))))