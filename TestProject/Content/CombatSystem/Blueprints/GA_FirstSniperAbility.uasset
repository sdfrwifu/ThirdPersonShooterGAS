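; GA_FirstSniperAbility is a gameplay ability for a sniper that deals damage over time in repeated ticks.
; Activation starts a looping timer whose event calls SniperAbilityDamage, which applies tick damage, counts ticks, and clears the timer at the maximum.
; The timer event passes no DamagedActor into that function, and the ability never calls EndAbility.
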(event `SniperAbilityDamageEvent`
  (`self.SniperAbilityDamage` null))

(event `self.K2_ActivateAbility`
  (if true
    (bind _returnvalue (`KismetSystemLibrary.K2_SetTimerDelegate` (delegate `SniperAbilityDamageEvent`) (`self.SniperAbilityTickTimeRate`) true))
    (set `self.SniperAbilityTimer` _returnvalue)))

(fn `SniperAbilityDamage`
  (params (DamagedActor :type "Actor Object Reference"))
  (locals (LocalSniperAbilityTickDamage :type "Float (double-precision)") (LocalMaxAmountOfTicks :type Integer))
  (`GameplayStatics.ApplyDamage` DamagedActor (`local.LocalSniperAbilityTickDamage`))
  (bind _result (`/Engine/EditorBlueprintResources/StandardMacros.IncrementInt` (`self.AbilityAmountOfTicks`))
    (:`  `
      (if (== _result (`local.LocalMaxAmountOfTicks`))
        (set `self.AbilityAmountOfTicks` 0)
        (`KismetSystemLibrary.K2_ClearAndInvalidateTimerHandle` (`self.SniperAbilityTimer`))))))