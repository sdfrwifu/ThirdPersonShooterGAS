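; Gameplay ability that fires the character's current weapon when aiming, loaded and not reloading, otherwise clearing the full-auto timer.
; A camera trace sets the aim point for a muzzle multi-trace, which damages character-interface actors.
; A height window above the victim's bottom socket selects the headshot multiplier.
; An active sniper first-ability tag adds looping timer damage ticks, then removes the tag and ends the ability.
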(event `self.K2_ActivateAbility`
  (bind _returnvalue (`self.GetAvatarActorFromActorInfo`))
  (bind _returnvalue_2 (`Actor.GetComponentByClass` _returnvalue "/Script/TestProject.MyAbilitySystemComponent"))
  (bind _returnvalue_3 (`SceneComponent.K2_GetComponentLocation` (`/Game/CombatSystem/Weapons/BP_BaseWeapon.Muzzle` (`self.CurrentWeapon`))))
  (`self.K2_CommitAbility`)
  (bind (_mainweapon _secondweapon _currentweapon) (message `/Game/CombatSystem/Interfaces/BPI_CharacterIntreface.GetCharacterWeapons` _returnvalue))
  (bind _output_get (set `self.CurrentWeapon` _currentweapon))
  (if (and (`GameplayTagAssetInterface.HasAllMatchingGameplayTags` _returnvalue_2 (`BlueprintGameplayTagLibrary.MakeLiteralGameplayTagContainer` (struct :`GameplayTags` (struct :`(TagName` "PlayerState.IsAiming") :`(TagName` "PlayerState.IsFireButtonPressed"))))) (> (`/Game/CombatSystem/Weapons/BP_BaseWeapon.CurrentAmountOfAmmo` _output_get) 0.0) (not (`GameplayTagAssetInterface.HasMatchingGameplayTag` _returnvalue_2 (struct :`TagName` "PlayerState.Reload"))))
    (`self.SpawnSoundAndFX`)
    (`self.AmmoSubtract`)
    (bind _outhit (`self.GetCameraTraceHit`))
    (bind (_bblockinghit _binitialoverlap _time _distance _location _impactpoint _normal _impactnormal _physmat _hitactor _hitcomponent _hitbonename _bonename _hititem _elementindex _faceindex _tracestart _traceend) (`GameplayStatics.BreakHitResult` _outhit))
    (bind _returnvalue_4 (- _location _returnvalue_3))
    (bind _outhits (`KismetSystemLibrary.LineTraceMulti` :`Start` _returnvalue_3 :`End` (`KismetMathLibrary.SelectVector` (+ (* (/ _returnvalue_4 (`KismetMathLibrary.VSize` _returnvalue_4)) (`self.ShootingDistanceMultiplayer`)) _location) _traceend _bblockinghit) :`TraceChannel` "TraceTypeQuery1" :`DrawDebugType` "ForDuration" :`bIgnoreSelf` false))
    (`self.TraceDamage` _outhits)
    (else
      (`KismetSystemLibrary.K2_ClearAndInvalidateTimerHandle` (`self.FullAutoTimer`)))))

(event `SniperFirstAbility`
  (`self.K2_CommitAbility`)
  (bind _returnvalue (`KismetSystemLibrary.K2_SetTimerDelegate` (delegate `SniperAbilityDamageEvent`) (`self.SniperAbilityTickTimeRate`) true))
  (set `self.SniperAbilityTimer` _returnvalue))

(event `SniperAbilityDamageEvent`
  (`self.SniperFirstAbilityDamage`))

(fn `GetCameraTraceHit`
  (returns (OutHit :type "HitResult Structure"))
  (bind _returnvalue (`GameplayStatics.GetPlayerCameraManager` 0))
  (bind _returnvalue_2 (`Actor.K2_GetActorLocation` _returnvalue))
  (bind _outhit (`KismetSystemLibrary.LineTraceSingle` :`Start` _returnvalue_2 :`End` (+ _returnvalue_2 (* (`Actor.GetActorForwardVector` _returnvalue) (`self.ShootingDistanceMultiplayer`))) :`TraceChannel` "TraceTypeQuery2" :`TraceColor` (struct :`R` 1.0 :`B` 0.826939 :`A` 1.0)))
  (return _outhit))

(fn `SniperFirstAbilityDamage`
  (locals (LocalSniperAbilityTickDamage :type "Float (double-precision)" :default 5.0) (LocalMaxAmountOfTicks :type Integer :default 4))
  (`GameplayStatics.ApplyDamage` (`self.DamagedActor`) (`local.LocalSniperAbilityTickDamage`))
  (bind _result (`/Engine/EditorBlueprintResources/StandardMacros.IncrementInt` (`self.SniperAbilityAmountOfTicks`))
    (:`  `
      (if (== _result (`local.LocalMaxAmountOfTicks`))
        (set `self.SniperAbilityAmountOfTicks` 0)
        (`KismetSystemLibrary.K2_ClearAndInvalidateTimerHandle` (`self.SniperAbilityTimer`))
        (`AbilitySystemBlueprintLibrary.RemoveLooseGameplayTags` (`self.GetAvatarActorFromActorInfo`) (`BlueprintGameplayTagLibrary.MakeLiteralGameplayTagContainer` (struct :`GameplayTags` (struct :`(TagName` "SniperCharacter.Abilities.First.IsActive")))))
        (`self.K2_EndAbility`)))))

(fn `TraceDamage`
  (params (OutHits :type "Array of HitResult Structure"))
  (locals (LocalLastHitActor :type "Actor Object Reference") (LocalBottomCharacterSocketName :type Name :default "bottom_Socket") (LocalHitComponent :type "PrimitiveComponent Object Reference"))
  (for _array_element OutHits
    (bind (_bblockinghit _binitialoverlap _time _distance _location _impactpoint _normal _impactnormal _physmat _hitactor _hitcomponent) (`GameplayStatics.BreakHitResult` _array_element))
    (if (`KismetSystemLibrary.DoesImplementInterface` _hitactor "/Game/CombatSystem/Interfaces/BPI_CharacterIntreface.BPI_CharacterIntreface_C")
      (message `/Game/CombatSystem/Interfaces/BPI_CharacterIntreface.SetHitLocation` (`self.GetAvatarActorFromActorInfo`) _location)
      (set `self.DamagedActor` _hitactor)
      (set `local.LocalHitComponent` _hitcomponent)
      (if (and (!= (`self.DamagedActor`) (`local.LocalLastHitActor`)) (not (`GameplayTagAssetInterface.HasMatchingGameplayTag` (`Actor.GetComponentByClass` (`self.GetAvatarActorFromActorInfo`) "/Script/TestProject.MyAbilitySystemComponent") (struct :`TagName` "PlayerState.IsDead"))))
        (bind _hitlocation (message `/Game/CombatSystem/Interfaces/BPI_CharacterIntreface.GetHitLocation` (`self.GetAvatarActorFromActorInfo`)))
        (bind _damagemultiplier (message `/Game/CombatSystem/Interfaces/BPI_CharacterIntreface.GetDamageMultiplier` (`self.GetAvatarActorFromActorInfo`)))
        (`GameplayStatics.ApplyDamage` (`self.DamagedActor`) (* (`/Game/CombatSystem/Weapons/BP_BaseWeapon.WeaponDamage` (`self.CurrentWeapon`)) (select `bool` (`KismetMathLibrary.InRange_FloatFloat` (.z (- _hitlocation (`SceneComponent.GetSocketLocation` (`local.LocalHitComponent`) (`local.LocalBottomCharacterSocketName`)))) 150.0 180.0) :`false` (`self.DefaultDamageMultiplier`) :`true` _damagemultiplier)))
        (`self.OnAddHitsInRowAmmo`)
        (set `local.LocalLastHitActor` (`self.DamagedActor`))
        (if (`GameplayTagAssetInterface.HasMatchingGameplayTag` (`Actor.GetComponentByClass` (`self.GetAvatarActorFromActorInfo`) "/Script/TestProject.MyAbilitySystemComponent") (struct :`TagName` "SniperCharacter.Abilities.First.IsActive"))
          (`self.SniperFirstAbility`)
          (else
            (`self.K2_EndAbility`)))))))