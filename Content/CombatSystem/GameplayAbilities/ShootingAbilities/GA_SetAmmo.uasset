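; Gameplay ability that refills the avatar's current weapon and updates the ammo display.
; On activation it commits, then sets the current weapon's ammo to its clip amount through interface messages on the avatar and weapon.
; It writes the new ammo count to the character HUD's ammo text and ends, but only ends if that HUD is valid.
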(event `self.K2_ActivateAbility`
  (`self.K2_CommitAbility`)
  (bind (_mainweapon _secondweapon _currentweapon) (message `/Game/CombatSystem/Interfaces/BPI_CharacterIntreface.GetCharacterWeapons` (`self.GetAvatarActorFromActorInfo`)))
  (message `/Game/CombatSystem/Interfaces/BPI_WeaponInterface.SetCurrentAmmo` _currentweapon (`/Game/CombatSystem/Weapons/BP_BaseWeapon.ClipAmount` _currentweapon))
  (`self.SetTextToWidget`))

(fn `SetTextToWidget`
  (bind _returnvalue (`self.GetAvatarActorFromActorInfo`))
  (bind _charcaterhud (message `/Game/CombatSystem/Interfaces/BPI_CharacterIntreface.GetCharacterHud` _returnvalue))
  (`/Engine/EditorBlueprintResources/StandardMacros.IsValid` _charcaterhud
    (:`Is Valid`
      (bind (_mainweapon _secondweapon _currentweapon) (message `/Game/CombatSystem/Interfaces/BPI_CharacterIntreface.GetCharacterWeapons` _returnvalue))
      (`TextBlock.SetText` (`/Game/CombatSystem/Hud/CharacterHud.AmmoAmount` _charcaterhud) (`KismetTextLibrary.Conv_DoubleToText` (`/Game/CombatSystem/Weapons/BP_BaseWeapon.CurrentAmountOfAmmo` _currentweapon) "HalfToEven"))
      (`self.K2_EndAbility`))))