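; Sniper shooting Gameplay Ability that extends a parent shooting ability with hit damage and a damage-over-time effect.
; TraceDamage applies weapon damage to character hits, using the shooter's multiplier when impact height above the bottom socket falls in a head-level band, and credits hits-in-a-row ammo.
; With the first-ability tag active, a looping timer repeats tick damage on the last target until the tick limit, then removes the tag and ends the ability.
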(event `self.K2_ActivateAbility`
  (`parent.K2_ActivateAbility`))

(event `SniperShootingAbility`
  (bind _returnvalue (`KismetSystemLibrary.K2_SetTimerDelegate` (delegate `SniperAbilityDamageEvent`) (`self.SniperAbilityTickTimeRate`) true))
  (set `self.SniperAbilityTimer` _returnvalue))

(event `SniperAbilityDamageEvent`
  (`self.SniperFirstAbilityDamage`))

(fn `SniperFirstAbilityDamage`
  (locals (LocalSniperAbilityTickDamage :type "Float (double-precision)" :default 5.0) (LocalMaxAmountOfTicks :type Integer :default 4))
  (`GameplayStatics.ApplyDamage` (`self.DamagedActor`) (`local.LocalSniperAbilityTickDamage`))
  (bind _result (`/Engine/EditorBlueprintResources/StandardMacros.IncrementInt` (`self.SniperAbilityAmountOfTicks`))
    (:`  `
      (if (== _result (`local.LocalMaxAmountOfTicks`))
        (set `self.SniperAbilityAmountOfTicks` 0)
        (`KismetSystemLibrary.K2_ClearAndInvalidateTimerHandle` (`self.SniperAbilityTimer`))
        (`AbilitySystemBlueprintLibrary.RemoveLooseGameplayTags` (`self.GetAvatarActorFromActorInfo`) (`BlueprintGameplayTagLibrary.MakeLiteralGameplayTagContainer` (struct :`GameplayTags` (struct :`(TagName` "SniperCharacter.Abilities.First.IsActive")))))
        (`self.K2_EndAbility`)))))

(fn `TraceDamage`
  (params (OutHits :type "Array of HitResult Structure (by ref)"))
  (locals (LocalHitComponent :type "PrimitiveComponent Object Reference") (LocalLastHitActor :type "Actor Object Reference") (LocalBottomCharacterSocketName :type Name :default "bottom_Socket"))
  (for _array_element OutHits
    (bind (_bblockinghit _binitialoverlap _time _distance _location _impactpoint _normal _impactnormal _physmat _hitactor _hitcomponent) (`GameplayStatics.BreakHitResult` _array_element))
    (if (`KismetSystemLibrary.DoesImplementInterface` _hitactor "/Game/CombatSystem/Interfaces/BPI_CharacterIntreface.BPI_CharacterIntreface_C")
      (message `/Game/CombatSystem/Interfaces/BPI_CharacterIntreface.SetHitLocation` (`self.GetAvatarActorFromActorInfo`) _location)
      (set `self.DamagedActor` _hitactor)
      (set `local.LocalHitComponent` _hitcomponent)
      (if (and (!= (`self.DamagedActor`) (`local.LocalLastHitActor`)) (not (`GameplayTagAssetInterface.HasMatchingGameplayTag` (`Actor.GetComponentByClass` (`self.GetAvatarActorFromActorInfo`) "/Script/TestProject.MyAbilitySystemComponent") (struct :`TagName` "PlayerState.IsDead"))))
        (bind _hitlocation (message `/Game/CombatSystem/Interfaces/BPI_CharacterIntreface.GetHitLocation` (`self.GetAvatarActorFromActorInfo`)))
        (bind _damagemultiplier (message `/Game/CombatSystem/Interfaces/BPI_CharacterIntreface.GetDamageMultiplier` (`self.GetAvatarActorFromActorInfo`)))
        (`GameplayStatics.ApplyDamage` (`self.DamagedActor`) (* (`/Game/CombatSystem/Weapons/BP_BaseWeapon.WeaponDamage` (`self.CurrentWeapon`)) (select `bool` (`KismetMathLibrary.InRange_FloatFloat` (.z (- _hitlocation (`SceneComponent.GetSocketLocation` (`local.LocalHitComponent`) (`local.LocalBottomCharacterSocketName`)))) 150.0 180.0) :`false` (`self.DefaultDamageMultiplier`) :`true` _damagemultiplier)))
        (`self.OnAddHitsInRowAmmo`)
        (set `local.LocalLastHitActor` (`self.DamagedActor`))
        (if (`GameplayTagAssetInterface.HasMatchingGameplayTag` (`Actor.GetComponentByClass` (`self.GetAvatarActorFromActorInfo`) "/Script/TestProject.MyAbilitySystemComponent") (struct :`TagName` "SniperCharacter.Abilities.First.IsActive"))
          (`self.SniperShootingAbility`)
          (else
            (`self.K2_EndAbility`))))))
  (`local.LocalLastHitActor`
    (:`then`)
    (:`else`
      (`self.K2_EndAbility`))))