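; Weapon reload gameplay ability for the StormTrooper character, overriding steps of a parent reload ability.
; Setting the weapon first sends a begin-reload message to the avatar.
; After the parent's ammo refill, it adds bonus rounds from the avatar's biggest hits-in-a-row ammo value.
; The montage play rate switches to an ability-specific rate while the StormTrooper's first-ability active tag is present.
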(fn `SetCurrentAmmo`
  (bind _currentweapon (`self.CurrentWeapon`))
  (`parent.SetCurrentAmmo`)
  (bind _ammotoadd (message `/Game/CombatSystem/Interfaces/BPI_StormTrooperInterface.GetBiggestHitsInRowAmmo` (`self.GetAvatarActorFromActorInfo`)))
  (message `/Game/CombatSystem/Interfaces/BPI_WeaponInterface.SetCurrentAmmo` _currentweapon (+ (`/Game/CombatSystem/Weapons/BP_BaseWeapon.CurrentAmountOfAmmo` _currentweapon) _ammotoadd)))

(fn `SetCurrentWeapon`
  (message `/Game/CombatSystem/Interfaces/BPI_StormTrooperInterface.WeaponBeginReload` (`self.GetAvatarActorFromActorInfo`))
  (`parent.SetCurrentWeapon`))

(fn `SetMontageStats`
  (returns (ReloadMontage :type "AnimMontage Object Reference") (MontageSectionName :type Name) (MontagePlayRate :type "Float (double-precision)"))
  (bind (_reloadmontage _montagesectionname) (`parent.SetMontageStats`))
  (return _reloadmontage _montagesectionname (`KismetMathLibrary.SelectFloat` (`self.AbilityMontagePlayRate`) (`self.DefaultMontagePlayRate`) (`GameplayTagAssetInterface.HasMatchingGameplayTag` (`Actor.GetComponentByClass` (`self.GetAvatarActorFromActorInfo`) "/Script/TestProject.MyAbilitySystemComponent") (struct :`TagName` "StormTrooperCharacter.Abilities.First.IsActive")))))