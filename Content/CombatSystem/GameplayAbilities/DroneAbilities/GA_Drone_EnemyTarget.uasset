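; Event-triggered gameplay ability that sends a drone after an enemy target supplied in the payload.
; It accepts only living characters other than the drone or its instigator, when no target is already set.
; A looping timer re-issues AI moves to the target's location, applying lock-on speed and a colour change.
; A second timer lerps rotation toward the target and clears the rotating tag, while move completion ends the ability.
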(event `self.K2_ActivateAbilityFromEvent`
  (params (EventData :type "GameplayEventData Structure (by ref)"))
  (set `self.DroneActor` (`self.GetAvatarActorFromActorInfo`))
  (`self.K2_CommitAbility`)
  (bind _asbp_drone_enemy_target_paylaod (cast `/Game/CombatSystem/GameplayAbilities/DroneAbilities/BP_Drone_EnemyTargetPaylaod` (`.OptionalObject` (break `GameplayEventData` EventData))))
  (bind _targetactor (`/Game/CombatSystem/GameplayAbilities/DroneAbilities/BP_Drone_EnemyTargetPaylaod.TargetActor` _asbp_drone_enemy_target_paylaod))
  (if (`self.IsTargetValidForAbility` _targetactor)
    (if (`self.CanTargetBeDamaged` _targetactor)
      (set `self.CurrentTarget` _targetactor)
      (`self.EventDroneMove`)
      (`KismetSystemLibrary.K2_SetTimerDelegate` (delegate `DroneMove`) 0.1 true)
      (else
        (`self.K2_EndAbility` :!label _label)))
    (else
      (goto _label))))

(event `DroneMove`
  (`self.EventDroneMove`))

(event `EventDroneMove`
  (`AITask_MoveTo.AIMoveTo` (`AIBlueprintHelperLibrary.GetAIController` (`self.DroneActor`)) (`Actor.K2_GetActorLocation` (`self.CurrentTarget`)) null 25.0 "Disable"
    (:`then`
      (bind _returnvalue (`KismetSystemLibrary.K2_SetTimerDelegate` (delegate `RotatingLerp`) (`self.RotateLerpTickTimeRate`) true))
      (`KismetSystemLibrary.K2_ClearAndInvalidateTimerHandle` (`self.RotateLerpTimer`))
      (set `self.RotateLerpTimer` _returnvalue)
      (set `FloatingPawnMovement.MaxSpeed` (`self.MaxDroneLockOnTargetSpeed`) (`Actor.GetComponentByClass` (`self.DroneActor`) "/Script/Engine.FloatingPawnMovement"))
      (message `/Game/CombatSystem/Interfaces/BPI_Drone.CallChangeDroneColor` (`self.DroneActor`)))
    (:`OnMoveFinished`
      (`self.K2_EndAbility`))))

(event `RotatingLerp`
  (`self.RotateToTarget`))

(fn `CanTargetBeDamaged`
  (params (TargetActor :type "Actor Object Reference"))
  (returns (ReturnValue :type Boolean))
  (return (and (not (`GameplayTagAssetInterface.HasMatchingGameplayTag` (`Actor.GetComponentByClass` TargetActor "/Script/TestProject.MyAbilitySystemComponent") (struct :`TagName` "Character.States.IsDead"))) (not (`KismetSystemLibrary.IsValid` (`self.CurrentTarget`))))))

(fn `IsTargetValidForAbility`
  (params (TargetActor :type "Actor Object Reference"))
  (returns (ReturnValue :type Boolean))
  (bind _droneactor (`self.DroneActor`))
  (return (and (!= _droneactor TargetActor) (!= TargetActor (`Actor.Instigator` _droneactor)) (`KismetSystemLibrary.DoesImplementInterface` TargetActor "/Game/CombatSystem/Interfaces/BPI_BaseCharacter.BPI_BaseCharacter_C"))))

(fn `RotateToTarget`
  (locals (LocalRotateAlphaLerpChangeRate :type "Float (double-precision)" :default 0.025) (LocalLerpEndAlpha :type "Float (double-precision)" :default 1.0) (LocalMaxRotateAlphaValue :type "Float (double-precision)" :default 1.0))
  (bind _droneactor (`self.DroneActor`))
  (bind _output_get (set `self.RotateAlpha` (`KismetMathLibrary.FClamp` (+ (`self.RotateAlpha`) (`local.LocalRotateAlphaLerpChangeRate`)) 0.0 (`local.LocalMaxRotateAlphaValue`))))
  (`Actor.K2_SetActorRotation` (`self.DroneActor`) (`KismetMathLibrary.RLerp` (`Actor.K2_GetActorRotation` _droneactor) (`KismetMathLibrary.FindLookAtRotation` (`Actor.K2_GetActorLocation` _droneactor) (`Actor.K2_GetActorLocation` (`self.CurrentTarget`))) _output_get true) false)
  (if (>= (`self.RotateAlpha`) (`local.LocalLerpEndAlpha`))
    (`KismetSystemLibrary.K2_ClearAndInvalidateTimerHandle` (`self.RotateLerpTimer`))
    (`AbilitySystemBlueprintLibrary.RemoveLooseGameplayTags` (`self.DroneActor`) (`BlueprintGameplayTagLibrary.MakeLiteralGameplayTagContainer` (struct :`GameplayTags` (struct :`(TagName` "Drone.States.IsRotating")))))))