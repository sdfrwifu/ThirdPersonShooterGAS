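; Gameplay ability that reloads the avatar's current rifle when not already reloading, no montage is playing and the clip isn't full.
; It adds reload and upper-body tags, then picks a montage and start section from the IsClipInserted tag and remaining ammo.
; Completion refills the clip, adds one round for non-empty reloads, clears IsClipInserted and updates the widget text.
; Interruption only removes the reload tags and ends the ability.
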(event `self.K2_ActivateAbility`
  (bind _returnvalue (`self.GetAvatarActorFromActorInfo`))
  (bind _currentweapon (`self.CurrentWeapon`))
  (bind _montagesectionname (`self.MontageSectionName`))
  (`self.SetCurrentWeapon`)
  (if (and (not (`GameplayTagAssetInterface.HasMatchingGameplayTag` (`Actor.GetComponentByClass` _returnvalue "/Script/TestProject.MyAbilitySystemComponent") (struct :`TagName` "PlayerState.Reload"))) (not (`AnimInstance.IsAnyMontagePlaying` (`SkeletalMeshComponent.GetAnimInstance` (`Actor.GetComponentByClass` _returnvalue "/Script/Engine.SkeletalMeshComponent")))) (not (>= (`/Game/CombatSystem/Weapons/BP_BaseWeapon.CurrentAmountOfAmmo` _currentweapon) (`/Game/CombatSystem/Weapons/BP_BaseWeapon.ClipAmount` _currentweapon))))
    (`AbilitySystemBlueprintLibrary.AddLooseGameplayTags` (`self.GetAvatarActorFromActorInfo`) (`BlueprintGameplayTagLibrary.MakeGameplayTagContainerFromArray` (`|MakeArray` (struct :`TagName` "PlayerState.Reload") (struct :`TagName` "PlayerState.IsUpperBody") :!type "GameplayTag Structure")))
    (bind (_reloadmontage _montagesectionname_2 _montageplayrate) (`self.SetMontageStats`))
    (`AbilityTask_PlayMontageAndWait.CreatePlayMontageAndWaitProxy` "None" _reloadmontage _montageplayrate _montagesectionname_2
      (:`OnCompleted`
        (`self.SetCurrentAmmo`)
        (if (or (== _montagesectionname "NoShutter") (== _montagesectionname "NoClipNoShutter"))
          (`/Engine/EditorBlueprintResources/StandardMacros.IncrementFloat` (`/Game/CombatSystem/Weapons/BP_BaseWeapon.CurrentAmountOfAmmo` (`self.CurrentWeapon`))
            (:`  `
              _)))
        (`AbilitySystemBlueprintLibrary.RemoveLooseGameplayTags` (`self.GetAvatarActorFromActorInfo`) (`BlueprintGameplayTagLibrary.MakeGameplayTagContainerFromArray` (`|MakeArray` (struct :`TagName` "PlayerState.Reload") (struct :`TagName` "PlayerState.IsUpperBody") :!type "GameplayTag Structure")))
        (`AbilitySystemBlueprintLibrary.RemoveLooseGameplayTags` (`self.GetAvatarActorFromActorInfo`) (`BlueprintGameplayTagLibrary.MakeLiteralGameplayTagContainer` (struct :`GameplayTags` (struct :`(TagName` "WeaponState.IsClipInserted")))))
        (`self.SetTextToWidget`)
        (`self.K2_EndAbility`))
      (:`OnInterrupted`
        (`AbilitySystemBlueprintLibrary.RemoveLooseGameplayTags` (`self.GetAvatarActorFromActorInfo`) (`BlueprintGameplayTagLibrary.MakeGameplayTagContainerFromArray` (`|MakeArray` (struct :`TagName` "PlayerState.Reload") (struct :`TagName` "PlayerState.IsUpperBody") :!type "GameplayTag Structure")))
        (`self.K2_EndAbility`)))))

(fn `SetCurrentAmmo`
  (bind _currentweapon (`self.CurrentWeapon`))
  (set `/Game/CombatSystem/Weapons/BP_BaseWeapon.CurrentAmountOfAmmo` (`/Game/CombatSystem/Weapons/BP_BaseWeapon.ClipAmount` _currentweapon) _currentweapon))

(fn `SetCurrentWeapon`
  (bind (_mainweapon _secondweapon _currentweapon) (message `/Game/CombatSystem/Interfaces/BPI_CharacterIntreface.GetCharacterWeapons` (`self.GetAvatarActorFromActorInfo`)))
  (set `self.CurrentWeapon` _currentweapon)
  (return))

(fn `SetMontageStats`
  (returns (ReloadMontage :type "AnimMontage Object Reference") (MontageSectionName :type Name) (MontagePlayRate :type "Float (double-precision)"))
  (bind _currentamountofammo (`/Game/CombatSystem/Weapons/BP_BaseWeapon.CurrentAmountOfAmmo` (`self.CurrentWeapon`)))
  (if (`GameplayTagAssetInterface.HasMatchingGameplayTag` (`Actor.GetComponentByClass` (`self.GetAvatarActorFromActorInfo`) "/Script/TestProject.MyAbilitySystemComponent") (struct :`TagName` "WeaponState.IsClipInserted"))
    (if (> _currentamountofammo 0.0)
      (set `self.MontageSectionName` "NoClipNoShutter")
      (else
        (set `self.MontageSectionName` "NoClip")))
    (set `self.ReloadMontage` "/Game/CombatSystem/Animations/MM_Rifle_Reload_Montage.MM_Rifle_Reload_Montage")
    (elif (> _currentamountofammo 0.0)
      (set `self.MontageSectionName` "NoShutter")
      (set `self.ReloadMontage` "/Game/CombatSystem/Animations/MM_Rifle_Reload_Montage1.MM_Rifle_Reload_Montage1")
      (else
        (set `self.MontageSectionName` "Default")
        (set `self.ReloadMontage` "/Game/CombatSystem/Animations/MM_Rifle_Reload_Montage.MM_Rifle_Reload_Montage"))))
  (return (`self.ReloadMontage`) (`self.MontageSectionName`) (`self.DefaultMontagePlayRate`)))