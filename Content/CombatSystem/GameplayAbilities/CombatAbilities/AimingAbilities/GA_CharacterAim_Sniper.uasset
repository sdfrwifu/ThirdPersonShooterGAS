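; Sniper variant of the character aim gameplay ability, adding scope view and weapon-dependent movement speed.
; Gameplay tags drive its functions: the pistol tag picks the stored max speed, and walk speed takes the higher of that and the default.
; HUD setup extends the parent, narrowing FOV and showing the scope image while scoping, otherwise the aim image.
; The speed update also restores default FOV if the scoping tag is present.
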(fn `SetAimingFOV`
  (locals (LocalScopingFOV :type "Float (single-precision)" :default 27.0))
  (bind _charcaterhud (message `/Game/CombatSystem/Interfaces/BPI_BaseCharacter.GetCharacterHud` (`self.GetAvatarActorFromActorInfo`)))
  (`/Engine/EditorBlueprintResources/StandardMacros.IsValid` _charcaterhud
    (:`Is Valid`
      (if (`GameplayTagAssetInterface.HasMatchingGameplayTag` (`Actor.GetComponentByClass` (`self.GetAvatarActorFromActorInfo`) "/Script/TestProject.MyAbilitySystemComponent") (struct :`TagName` "Character.Sniper.States.IsScoping"))
        (bind _cameracomponent (message `/Game/CombatSystem/Interfaces/BPI_BaseCharacter.GetCharacterCamera` (`self.GetAvatarActorFromActorInfo`)))
        (`CameraComponent.SetFieldOfView` _cameracomponent (`local.LocalScopingFOV`))
        (bind _aimimage (`/Game/CombatSystem/Hud/CharacterHud.AimImage` _charcaterhud))
        (`Widget.SetVisibility` _aimimage "Hidden")
        (`Widget.SetVisibility` (`/Game/CombatSystem/Hud/CharacterHud.ScopeImage` _charcaterhud) "Visible")
        (else
          (`Widget.SetVisibility` (`/Game/CombatSystem/Hud/CharacterHud.ScopeImage` _charcaterhud) "Hidden")
          (`Widget.SetVisibility` _aimimage "Visible"))))))

(fn `SetHudSettings`
  (`parent.SetHudSettings`)
  (`self.SetAimingFOV`))

(fn `SetMaxCharacterSpeed`
  (bind _returnvalue (`Actor.GetComponentByClass` (`self.GetAvatarActorFromActorInfo`) "/Script/TestProject.MyAbilitySystemComponent"))
  (message `/Game/CombatSystem/Interfaces/BPI_BaseCharacter.SetCurrentMaxCharacterSpeed` (`self.GetAvatarActorFromActorInfo`) (`KismetMathLibrary.SelectFloat` (`self.MaxPistolCharacterSpeed`) (`self.MaxDefaultCharacterSpeed`) (`GameplayTagAssetInterface.HasMatchingGameplayTag` _returnvalue (struct :`TagName` "Character.Sniper.States.IsCurrentWeaponPistol"))))
  (if (`GameplayTagAssetInterface.HasMatchingGameplayTag` _returnvalue (struct :`TagName` "Character.Sniper.States.IsScoping"))
    (bind (_cameracomponent _defaultfov) (message `/Game/CombatSystem/Interfaces/BPI_BaseCharacter.GetCharacterCamera` (`self.GetAvatarActorFromActorInfo`)))
    (`CameraComponent.SetFieldOfView` _cameracomponent _defaultfov)))

(fn `SetWalkSpeed`
  (bind _returnvalue (`self.GetAvatarActorFromActorInfo`))
  (`self.SetMaxCharacterSpeed`)
  (bind _currentmaxspeed (message `/Game/CombatSystem/Interfaces/BPI_BaseCharacter.GetCurrentMaxCharacterSpeed` _returnvalue))
  (set `CharacterMovementComponent.MaxWalkSpeed` (`KismetMathLibrary.SelectFloat` _currentmaxspeed (`self.MaxDefaultCharacterSpeed`) (> _currentmaxspeed (`self.MaxDefaultCharacterSpeed`))) (`Actor.GetComponentByClass` _returnvalue "/Script/Engine.CharacterMovementComponent")))