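; Gameplay ability that switches the character into or out of aiming based on the IsAiming tag, skipped during weapon swaps.
; Aiming sets walk speed, controller-driven rotation and the aim HUD; not aiming restores speed and movement-oriented rotation, hides the HUD and resets FOV.
; A looping timer lerps the spring arm socket offset toward the current state, clearing itself at either end threshold.
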(event `self.K2_ActivateAbility`
  (bind _returnvalue (`Actor.GetComponentByClass` (`self.GetAvatarActorFromActorInfo`) "/Script/TestProject.MyAbilitySystemComponent"))
  (if (not (`GameplayTagAssetInterface.HasMatchingGameplayTag` _returnvalue (struct :`TagName` "WeaponState.IsSwapping")))
    (if (`GameplayTagAssetInterface.HasMatchingGameplayTag` _returnvalue (struct :`TagName` "Character.States.IsAiming"))
      (`self.AimingSettings`)
      (else
        (`self.NotAimingSettings`)))
    (bind _returnvalue_2 (`KismetSystemLibrary.K2_SetTimerDelegate` (delegate `CameraLerp`) (`self.AimingLerpTickTimeRate`) true))
    (set `self.AimingTimer` _returnvalue_2)))

(event `CameraLerp`
  (`self.AimCameraChange` (* (`self.AimingLerpChangeRate`) (`KismetMathLibrary.SelectFloat` 1.0 -1.0 (`GameplayTagAssetInterface.HasMatchingGameplayTag` (`Actor.GetComponentByClass` (`self.GetAvatarActorFromActorInfo`) "/Script/TestProject.MyAbilitySystemComponent") (struct :`TagName` "Character.States.IsAiming"))))))

(fn `AimCameraChange`
  (params (AimingLerpChangeRate :type "Float (double-precision)"))
  (locals (LocalDefaultSpringArmOffset :type "Vector Structure") (LocalAimingSpringArmOffset :type "Vector Structure" :default (270.0 80.0 70.0)) (LocalLerpEndAlpha :type "Float (double-precision)" :default 1.0) (LocalLerpEndAlphaNotAiming :type "Float (double-precision)"))
  (bind _aimingalpha (`self.AimingAlpha`))
  (bind _output_get (set `self.AimingAlpha` (`KismetMathLibrary.FClamp` (+ (`self.AimingAlpha`) AimingLerpChangeRate))))
  (bind (_cameracomponent _defaultfov _springarmcomponent) (message `/Game/CombatSystem/Interfaces/BPI_CharacterIntreface.GetCharacterCamera` (`self.GetAvatarActorFromActorInfo`)))
  (set `SpringArmComponent.SocketOffset` (`KismetMathLibrary.VLerp` (`local.LocalDefaultSpringArmOffset`) (`local.LocalAimingSpringArmOffset`) (`KismetMathLibrary.FClamp` _output_get)) _springarmcomponent)
  (if (>= _aimingalpha (`local.LocalLerpEndAlpha`))
    (`KismetSystemLibrary.K2_ClearAndInvalidateTimerHandle` (`self.AimingTimer`) :!label _label)
    (elif (<= _aimingalpha (`local.LocalLerpEndAlphaNotAiming`))
      (goto _label))))

(fn `AimingSettings`
  (locals (LocalMaxAimingCharacterSpeed :type "Float (double-precision)" :default 120.0))
  (bind _returnvalue (`Actor.GetComponentByClass` (`self.GetAvatarActorFromActorInfo`) "/Script/Engine.CharacterMovementComponent"))
  (set `CharacterMovementComponent.MaxWalkSpeed` (`local.LocalMaxAimingCharacterSpeed`) _returnvalue)
  (set `CharacterMovementComponent.bOrientRotationToMovement` false _returnvalue)
  (set `CharacterMovementComponent.bUseControllerDesiredRotation` true _returnvalue)
  (bind _charcaterhud (message `/Game/CombatSystem/Interfaces/BPI_CharacterIntreface.GetCharacterHud` (`self.GetAvatarActorFromActorInfo`)))
  (`Widget.SetVisibility` _charcaterhud "Visible")
  (`Widget.SetVisibility` (`/Game/CombatSystem/Hud/CharacterHud.ScopeImage` _charcaterhud) "Hidden")
  (`Widget.SetVisibility` (`/Game/CombatSystem/Hud/CharacterHud.AimImage` _charcaterhud) "Visible"))

(fn `NotAimingSettings`
  (bind _returnvalue (`Actor.GetComponentByClass` (`self.GetAvatarActorFromActorInfo`) "/Script/Engine.CharacterMovementComponent"))
  (`self.SetWalkSpeed`)
  (set `CharacterMovementComponent.bOrientRotationToMovement` true _returnvalue)
  (set `CharacterMovementComponent.bUseControllerDesiredRotation` false _returnvalue)
  (bind _charcaterhud (message `/Game/CombatSystem/Interfaces/BPI_CharacterIntreface.GetCharacterHud` (`self.GetAvatarActorFromActorInfo`)))
  (`Widget.SetVisibility` _charcaterhud "Hidden")
  (bind (_cameracomponent _defaultfov) (message `/Game/CombatSystem/Interfaces/BPI_CharacterIntreface.GetCharacterCamera` (`self.GetAvatarActorFromActorInfo`)))
  (`CameraComponent.SetFieldOfView` _cameracomponent _defaultfov))

(fn `SetWalkSpeed`
  (bind _currentmaxcharacterspeed (`self.CurrentMaxCharacterSpeed`))
  (set `CharacterMovementComponent.MaxWalkSpeed` (`KismetMathLibrary.SelectFloat` _currentmaxcharacterspeed (`self.MaxDefaultCharacterSpeed`) (> _currentmaxcharacterspeed (`self.MaxDefaultCharacterSpeed`))) (`Actor.GetComponentByClass` (`self.GetAvatarActorFromActorInfo`) "/Script/Engine.CharacterMovementComponent")))