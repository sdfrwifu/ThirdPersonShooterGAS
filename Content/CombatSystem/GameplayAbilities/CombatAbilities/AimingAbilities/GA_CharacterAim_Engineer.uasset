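; Engineer variant of the character aim gameplay ability, supplying the class-specific walk speed logic.
; SetWalkSpeed sets MaxWalkSpeed from the default character speed, applying the drone aura and movement ability multipliers when the matching Engineer state tags are on the Ability System Component.
; Nested float selects let both multipliers stack.
; The activate and end events are disabled stubs, leaving the aim flow to the parent class.
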(fn `SetWalkSpeed`
  (locals (LocalInDroneAuraSpeedMultipluier :type "Float (double-precision)" :default 1.1) (LocalMovementAbilitySpeedMultiplier :type "Float (double-precision)" :default 1.5))
  (bind _maxdefaultcharacterspeed (`self.MaxDefaultCharacterSpeed`))
  (bind _returnvalue (`KismetMathLibrary.SelectFloat` (* _maxdefaultcharacterspeed (`local.LocalInDroneAuraSpeedMultipluier`)) _maxdefaultcharacterspeed (`GameplayTagAssetInterface.HasMatchingGameplayTag` (`self.AbilitySystemComponent`) (struct :`TagName` "Character.Engineer.States.IsInDroneAura"))))
  (set `CharacterMovementComponent.MaxWalkSpeed` (`KismetMathLibrary.SelectFloat` (* _returnvalue (`local.LocalMovementAbilitySpeedMultiplier`)) _returnvalue (`GameplayTagAssetInterface.HasMatchingGameplayTag` (`self.AbilitySystemComponent`) (struct :`TagName` "Character.Engineer.States.IsMovementAbilityActive"))) (`self.MovementComponent`)))