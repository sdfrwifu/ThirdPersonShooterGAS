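; Base gameplay ability for character aiming, which ends immediately if the character is falling or swapping weapons.
; Aiming changes walk speed, switches rotation to follow the controller and shows the aim HUD.
; A looping timer lerps the spring arm socket offset, with rate chosen by the IsAiming tag.
; Removing that tag restores movement, HUD and FOV, then restarts the lerp, ending the ability once it finishes.
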(event `ActivateAimingTimer`
  (bind _returnvalue (`KismetSystemLibrary.K2_SetTimerDelegate` (delegate `CameraLerp`) (`self.AimingLerpTickTimeRate`) true))
  (set `self.AimingTimer` _returnvalue))

(event `CameraLerp`
  (`self.ActivateCameraLerp`))

(event `self.K2_ActivateAbility`
  (bind _returnvalue (`Actor.GetComponentByClass` (`self.GetAvatarActorFromActorInfo`) "/Script/Engine.CharacterMovementComponent"))
  (bind _returnvalue_2 (`Actor.GetComponentByClass` (`self.GetAvatarActorFromActorInfo`) "/Script/TestProject.MyAbilitySystemComponent"))
  (if (and (not (`NavMovementComponent.IsFalling` _returnvalue)) (`KismetSystemLibrary.IsValid` _returnvalue) (`KismetSystemLibrary.IsValid` _returnvalue_2))
    (set `self.AbilitySystemComponent` _returnvalue_2)
    (set `self.MovementComponent` _returnvalue)
    (`AbilityTask_WaitGameplayTagRemoved.WaitGameplayTagRemove` (struct :`TagName` "Character.States.IsAiming") null
      (:`then`
        (if (not (`GameplayTagAssetInterface.HasMatchingGameplayTag` (`self.AbilitySystemComponent`) (struct :`TagName` "WeaponState.IsSwapping")))
          (`self.AimingSettings`)
          (`self.ActivateAimingTimer`)
          (else
            (`self.K2_EndAbility`))))
      (:`Removed`
        (`KismetSystemLibrary.K2_ClearAndInvalidateTimerHandle` (`self.AimingTimer`))
        (`self.NotAimingSettings`)
        (`self.ActivateAimingTimer`)))
    (else
      (`self.K2_EndAbility`))))

(fn `ActivateCameraLerp`
  (locals (LocalAimingChangeRateMuliplier :type "Float (double-precision)" :default 1.0) (LocalNotAimingChangeRateMuliplier :type "Float (double-precision)" :default -1.0))
  (bind _returnvalue (`GameplayTagAssetInterface.HasMatchingGameplayTag` (`self.AbilitySystemComponent`) (struct :`TagName` "Character.States.IsAiming")))
  (if _returnvalue
    (`self.AimingSettings`))
  (`self.AimCameraChange` (* (`self.AimingLerpChangeRate`) (`KismetMathLibrary.SelectFloat` (`local.LocalAimingChangeRateMuliplier`) (`local.LocalNotAimingChangeRateMuliplier`) _returnvalue))))

(fn `AimCameraChange`
  (params (AimingLerpChangeRate :type "Float (double-precision)"))
  (locals (LocalDefaultSpringArmOffset :type "Vector Structure") (LocalAimingSpringArmOffset :type "Vector Structure" :default (270.0 80.0 70.0)) (LocalLerpEndAlpha :type "Float (double-precision)" :default 1.0) (LocalLerpEndAlphaNotAiming :type "Float (double-precision)") (LocalMaxAlphaValue :type "Float (double-precision)" :default 1.0))
  (set `self.AimingAlpha` (`KismetMathLibrary.FClamp` (+ (`self.AimingAlpha`) AimingLerpChangeRate) 0.0 (`local.LocalMaxAlphaValue`)))
  (bind (_cameracomponent _defaultfov _springarmcomponent) (message `/Game/CombatSystem/Interfaces/BPI_BaseCharacter.GetCharacterCamera` (`self.GetAvatarActorFromActorInfo`)))
  (set `SpringArmComponent.SocketOffset` (`KismetMathLibrary.VLerp` (`local.LocalDefaultSpringArmOffset`) (`local.LocalAimingSpringArmOffset`) (`KismetMathLibrary.FClamp` (`self.AimingAlpha`) 0.0 (`local.LocalMaxAlphaValue`))) _springarmcomponent)
  (if (>= (`self.AimingAlpha`) (`local.LocalLerpEndAlpha`))
    (`KismetSystemLibrary.K2_ClearAndInvalidateTimerHandle` (`self.AimingTimer`) :!label _label)
    (if (not (`GameplayTagAssetInterface.HasMatchingGameplayTag` (`self.AbilitySystemComponent`) (struct :`TagName` "Character.States.IsAiming")))
      (`self.K2_EndAbility`))
    (elif (<= (`self.AimingAlpha`) (`local.LocalLerpEndAlphaNotAiming`))
      (goto _label))))

(fn `AimingSettings`
  (locals (LocalMaxAimingCharacterSpeed :type "Float (double-precision)" :default 120.0))
  (bind _movementcomponent (`self.MovementComponent`))
  (set `CharacterMovementComponent.MaxWalkSpeed` (`local.LocalMaxAimingCharacterSpeed`) _movementcomponent)
  (set `CharacterMovementComponent.bOrientRotationToMovement` false _movementcomponent)
  (set `CharacterMovementComponent.bUseControllerDesiredRotation` true _movementcomponent)
  (`self.SetHudSettings`))

(fn `NotAimingSettings`
  (bind _movementcomponent (`self.MovementComponent`))
  (`self.SetWalkSpeed`)
  (set `CharacterMovementComponent.bOrientRotationToMovement` true _movementcomponent)
  (set `CharacterMovementComponent.bUseControllerDesiredRotation` false _movementcomponent)
  (bind _charcaterhud (message `/Game/CombatSystem/Interfaces/BPI_BaseCharacter.GetCharacterHud` (`self.GetAvatarActorFromActorInfo`)))
  (`Widget.SetVisibility` _charcaterhud "Hidden")
  (bind (_cameracomponent _defaultfov) (message `/Game/CombatSystem/Interfaces/BPI_BaseCharacter.GetCharacterCamera` (`self.GetAvatarActorFromActorInfo`)))
  (`CameraComponent.SetFieldOfView` _cameracomponent _defaultfov))

(fn `SetHudSettings`
  (bind _charcaterhud (message `/Game/CombatSystem/Interfaces/BPI_BaseCharacter.GetCharacterHud` (`self.GetAvatarActorFromActorInfo`)))
  (`Widget.SetVisibility` _charcaterhud "Visible")
  (`Widget.SetVisibility` (`/Game/CombatSystem/Hud/CharacterHud.ScopeImage` _charcaterhud) "Hidden")
  (`Widget.SetVisibility` (`/Game/CombatSystem/Hud/CharacterHud.AimImage` _charcaterhud) "Visible"))

(fn `SetWalkSpeed`
  (set `CharacterMovementComponent.MaxWalkSpeed` (`self.MaxDefaultCharacterSpeed`) (`self.MovementComponent`)))