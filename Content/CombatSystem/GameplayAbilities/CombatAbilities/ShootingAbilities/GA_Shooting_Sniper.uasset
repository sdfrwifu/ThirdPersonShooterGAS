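; Sniper shooting ability that extends its parent's trace damage with a fire-rate cooldown and a first-ability bonus shot.
; TraceDamage runs the parent logic, then applies the cooldown effect, if not already active, using the weapon's fire rate as a SetByCaller magnitude.
; An active first-ability tag is consumed to apply its damage effect to the damaged actor.
; Otherwise it clears the last hit actor and adds the CantFire tag.
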(event `self.K2_ActivateAbility`
  (`parent.K2_ActivateAbility`))

(event `self.K2_OnEndAbility`
  (params (bWasCancelled :type Boolean))
  (`parent.K2_OnEndAbility` bWasCancelled))

(fn `TraceDamage`
  (params (OutHits :type "Array of HitResult Structure (by ref)"))
  (locals (LocalHitComponent :type "PrimitiveComponent Object Reference") (LocalBottomCharacterSocketName :type Name :default "bottom_Socket"))
  (`parent.TraceDamage` OutHits)
  (if (not (`GameplayTagAssetInterface.HasMatchingGameplayTag` (`self.AbilitySystemComponent`) (struct :`TagName` "SniperCharacter.Abilities.Shooting.Cooldown")))
    (bind _returnvalue (`AbilitySystemBlueprintLibrary.AssignTagSetByCallerMagnitude` (`self.MakeOutgoingGameplayEffectSpec` (`self.AbilityGameplayEffectCooldown`)) (struct :`TagName` "SniperCharacter.Abilities.Shooting.Data") (`/Game/CombatSystem/Weapons/BP_BaseWeapon.WeaponFireRate` (`self.CurrentWeapon`))))
    (`self.K2_ApplyGameplayEffectSpecToOwner` _returnvalue))
  (if (`GameplayTagAssetInterface.HasMatchingGameplayTag` (`self.AbilitySystemComponent`) (struct :`TagName` "SniperCharacter.Abilities.First.IsActive"))
    (`AbilitySystemBlueprintLibrary.RemoveLooseGameplayTags` (`self.GetAvatarActorFromActorInfo`) (`BlueprintGameplayTagLibrary.MakeLiteralGameplayTagContainer` (struct :`GameplayTags` (struct :`(TagName` "SniperCharacter.Abilities.First.IsActive")))))
    (`AbilitySystemComponent.BP_ApplyGameplayEffectToSelf` :`self` (`Actor.GetComponentByClass` (`self.DamagedActor`) "/Script/TestProject.MyAbilitySystemComponent") :`GameplayEffectClass` "/Game/CombatSystem/GameplayAbilities/SniperAbilities/FirstAbility/GE_FirstSniperAbilityDamage.GE_FirstSniperAbilityDamage_C")
    (else
      (set `self.LastHitActor` null)
      (if (not (`GameplayTagAssetInterface.HasMatchingGameplayTag` (`self.AbilitySystemComponent`) (struct :`TagName` "Character.States.CantFire")))
        (`AbilitySystemBlueprintLibrary.AddLooseGameplayTags` (`self.GetAvatarActorFromActorInfo`) (`BlueprintGameplayTagLibrary.MakeLiteralGameplayTagContainer` (struct :`GameplayTags` (struct :`(TagName` "Character.States.CantFire")))))))))