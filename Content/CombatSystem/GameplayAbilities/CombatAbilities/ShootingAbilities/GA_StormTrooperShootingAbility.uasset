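; Storm Trooper shooting gameplay ability that extends a parent ability with hits-in-row ammo tracking.
; Applying damage sends a hits-in-row ammo message to the avatar and adds a non-replicated enemy-damaged tag.
; After the parent trace, it commits the cooldown and runs the end step, which clears the damaged actor or, if none exists, sends the avatar an "in structure" ammo message.
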(event `self.K2_ActivateAbility`
  (`parent.K2_ActivateAbility`))

(event `self.K2_OnEndAbility`
  (params (bWasCancelled :type Boolean))
  (`parent.K2_OnEndAbility` bWasCancelled))

(fn `ApplyDamage`
  (params (DamagedActor :type "Actor Object Reference") (BaseDamage :type "Float (single-precision)"))
  (bind _returnvalue (`self.GetAvatarActorFromActorInfo`))
  (`parent.ApplyDamage` DamagedActor BaseDamage)
  (message `/Game/CombatSystem/Interfaces/BPI_StormTrooperInterface.AddHitsInRowAmmo` _returnvalue)
  (`AbilitySystemBlueprintLibrary.AddLooseGameplayTags` _returnvalue (`BlueprintGameplayTagLibrary.MakeLiteralGameplayTagContainer` (struct :`GameplayTags` (struct :`(TagName` "Character.States.IsEnemyDamaged"))))))

(fn `TraceDamage`
  (params (OutHits :type "Array of HitResult Structure (by ref)"))
  (`parent.TraceDamage` OutHits)
  (`self.K2_CommitAbilityCooldown` false)
  (`self.TraceDamageEndAbility`)
  (return))

(fn `TraceDamageEndAbility`
  (`/Engine/EditorBlueprintResources/StandardMacros.IsValid` (`self.DamagedActor`)
    (:`Is Valid`
      (set `self.DamagedActor` null))
    (:`Is Not Valid`
      (message `/Game/CombatSystem/Interfaces/BPI_StormTrooperInterface.AddHitsInRowAmmoInStructure` (`self.GetAvatarActorFromActorInfo`))))
  (`parent.TraceDamageEndAbility`))