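; Engineer shooting gameplay ability that fires a shotgun-style blast, building on a parent shooting ability.
; CreateMultiLineTrace fires several randomly spread line traces from the weapon muzzle toward the aim point, passing each result to TraceDamage for parent damage handling and cooldown commit.
; While the engineer's first-ability tag is active, it uses an alternate spread multiplier and counts shots, removing the tag once the limit is reached.
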(event `self.K2_ActivateAbility`
  (`parent.K2_ActivateAbility`))

(event `self.K2_OnEndAbility`
  (params (bWasCancelled :type Boolean))
  (`parent.K2_OnEndAbility` bWasCancelled))

(fn `CreateMultiLineTrace`
  (params (Hit :type "HitResult Structure (by ref)"))
  (locals (LocalMinLineTraceSpread :type "Float (double-precision)" :default -750.0) (LocalMaxLineTraceSpread :type "Float (double-precision)" :default 750.0) (LocalMaxAmountOfShotsAbility :type Integer :default 5))
  (bind (_bblockinghit _binitialoverlap _time _distance _location _impactpoint _normal _impactnormal _physmat _hitactor _hitcomponent _hitbonename _bonename _hititem _elementindex _faceindex _tracestart _traceend) (`GameplayStatics.BreakHitResult` Hit))
  (bind _localminlinetracespread (`local.LocalMinLineTraceSpread`))
  (bind _localmaxlinetracespread (`local.LocalMaxLineTraceSpread`))
  (bind _returnvalue (`SceneComponent.K2_GetComponentLocation` (`/Game/CombatSystem/Weapons/BP_BaseWeapon.Muzzle` (`self.CurrentWeapon`))))
  (bind _returnvalue_2 (select `bool` (`GameplayTagAssetInterface.HasMatchingGameplayTag` (`self.AbilitySystemComponent`) (struct :`TagName` "EngineerCharacter.Abilities.First.IsActive")) :`false` (`self.EngineerSpreadMultiplier`) :`true` (`self.AbilityEngineerSpreadMultiplier`)))
  (bind _returnvalue_3 (- _location _returnvalue))
  (if (and (>= (`self.AmountOfShotsAbility`) (`local.LocalMaxAmountOfShotsAbility`)) (`GameplayTagAssetInterface.HasMatchingGameplayTag` (`self.AbilitySystemComponent`) (struct :`TagName` "EngineerCharacter.Abilities.First.IsActive")))
    (`AbilitySystemBlueprintLibrary.RemoveLooseGameplayTags` (`self.GetAvatarActorFromActorInfo`) (`BlueprintGameplayTagLibrary.MakeLiteralGameplayTagContainer` (struct :`GameplayTags` (struct :`(TagName` "EngineerCharacter.Abilities.First.IsActive")))))
    (set `self.AmountOfShotsAbility` 0))
  (for _ (range (+ (`self.EnginnerBlastAmount`) 1))
    (bind _outhits (`KismetSystemLibrary.LineTraceMulti` :`Start` _returnvalue :`End` (+ (`KismetMathLibrary.SelectVector` (+ (* (/ _returnvalue_3 (`KismetMathLibrary.VSize` _returnvalue_3)) (`self.ShootingDistanceMultiplayer`)) _location) _traceend _bblockinghit) (`KismetMathLibrary.MakeVector` (* (`KismetMathLibrary.RandomFloatInRange` _localminlinetracespread _localmaxlinetracespread) _returnvalue_2) (* (`KismetMathLibrary.RandomFloatInRange` _localminlinetracespread _localmaxlinetracespread) _returnvalue_2) (* (`KismetMathLibrary.RandomFloatInRange` _localminlinetracespread _localmaxlinetracespread) _returnvalue_2))) :`TraceChannel` "TraceTypeQuery1" :`DrawDebugType` "ForDuration" :`bIgnoreSelf` false))
    (`self.TraceDamage` _outhits))
  (if (`GameplayTagAssetInterface.HasMatchingGameplayTag` (`self.AbilitySystemComponent`) (struct :`TagName` "EngineerCharacter.Abilities.First.IsActive"))
    (`/Engine/EditorBlueprintResources/StandardMacros.IncrementInt` (`self.AmountOfShotsAbility`)
      (:`  `
        _)))
  (`self.K2_EndAbility`))

(fn `TraceDamage`
  (params (OutHits :type "Array of HitResult Structure (by ref)"))
  (`parent.TraceDamage` OutHits)
  (`self.K2_CommitAbilityCooldown` false)
  (`self.TraceDamageEndAbility`)
  (return))

(fn `TraceDamageEndAbility`
  (`parent.TraceDamageEndAbility`))