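; Base gameplay ability for full-auto gun fire, repeating shots on a looping timer at the weapon's fire rate.
; Shots continue while aiming with ammo and not reloading; otherwise the timer clears and the ability ends.
; A camera trace sets the aim point for a muzzle multi-trace.
; Character hits take weapon damage, multiplied by height above a bottom socket, skipping the last damaged actor.
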(event `self.K2_ActivateAbility`
  (`self.K2_CommitAbility`)
  (bind _output_get (set `self.AbilitySystemComponent` (`Actor.GetComponentByClass` (`self.GetAvatarActorFromActorInfo`) "/Script/TestProject.MyAbilitySystemComponent")))
  (if (and (not (`GameplayTagAssetInterface.HasMatchingGameplayTag` _output_get (struct :`TagName` "PlayerState.Reload"))) (not (`KismetSystemLibrary.K2_IsTimerActiveHandle` (`self.FullAutoTimer`))))
    (`self.MultiTraceFire`)
    (bind _returnvalue (`KismetSystemLibrary.K2_SetTimerDelegate` (delegate `TimerEventMultiTrace`) (`/Game/CombatSystem/Weapons/BP_BaseWeapon.WeaponFireRate` (`self.CurrentWeapon`)) true))
    (set `self.FullAutoTimer` _returnvalue)))

(event `TimerEventMultiTrace`
  (`self.MultiTraceFire`))

(fn `ApplyDamage`
  (params (DamagedActor :type "Actor Object Reference") (BaseDamage :type "Float (single-precision)"))
  (`GameplayStatics.ApplyDamage` DamagedActor BaseDamage))

(fn `CreateMultiLineTrace`
  (params (Hit :type "HitResult Structure (by ref)"))
  (bind (_bblockinghit _binitialoverlap _time _distance _location _impactpoint _normal _impactnormal _physmat _hitactor _hitcomponent _hitbonename _bonename _hititem _elementindex _faceindex _tracestart _traceend) (`GameplayStatics.BreakHitResult` Hit))
  (bind _returnvalue (`SceneComponent.K2_GetComponentLocation` (`/Game/CombatSystem/Weapons/BP_BaseWeapon.Muzzle` (`self.CurrentWeapon`))))
  (bind _returnvalue_2 (- _location _returnvalue))
  (bind _outhits (`KismetSystemLibrary.LineTraceMulti` :`Start` _returnvalue :`End` (`KismetMathLibrary.SelectVector` (+ (* (/ _returnvalue_2 (`KismetMathLibrary.VSize` _returnvalue_2)) (`self.ShootingDistanceMultiplayer`)) _location) _traceend _bblockinghit) :`TraceChannel` "TraceTypeQuery1" :`DrawDebugType` "ForDuration" :`bIgnoreSelf` false))
  (`self.TraceDamage` _outhits))

(fn `GetCameraTraceHit`
  (returns (OutHit :type "HitResult Structure"))
  (bind _returnvalue (`GameplayStatics.GetPlayerCameraManager` 0))
  (bind _returnvalue_2 (`Actor.K2_GetActorLocation` _returnvalue))
  (bind _outhit (`KismetSystemLibrary.LineTraceSingle` :`Start` _returnvalue_2 :`End` (+ _returnvalue_2 (* (`Actor.GetActorForwardVector` _returnvalue) (`self.ShootingDistanceMultiplayer`))) :`TraceChannel` "TraceTypeQuery2" :`TraceColor` (struct :`R` 1.0 :`B` 0.826939 :`A` 1.0)))
  (return _outhit))

(fn `GetCanBeDamaged`
  (returns (ReturnValue :type Boolean))
  (return (and (!= (`self.DamagedActor`) (`self.LastHitActor`)) (not (`GameplayTagAssetInterface.HasMatchingGameplayTag` (`self.AbilitySystemComponent`) (struct :`TagName` "PlayerState.IsDead"))))))

(fn `MultiTraceFire`
  (bind (_mainweapon _secondweapon _currentweapon) (message `/Game/CombatSystem/Interfaces/BPI_CharacterIntreface.GetCharacterWeapons` (`self.GetAvatarActorFromActorInfo`)))
  (bind _output_get (set `self.CurrentWeapon` _currentweapon))
  (if (and (`GameplayTagAssetInterface.HasAllMatchingGameplayTags` (`self.AbilitySystemComponent`) (`BlueprintGameplayTagLibrary.MakeLiteralGameplayTagContainer` (struct :`GameplayTags` (struct :`(TagName` "PlayerState.IsAiming") :`(TagName` "PlayerState.IsFireButtonPressed"))))) (> (`/Game/CombatSystem/Weapons/BP_BaseWeapon.CurrentAmountOfAmmo` _output_get) 0.0) (not (`GameplayTagAssetInterface.HasMatchingGameplayTag` (`self.AbilitySystemComponent`) (struct :`TagName` "PlayerState.Reload"))))
    (`self.SpawnSoundAndFX`)
    (`self.AmmoSubtract`)
    (bind _outhit (`self.GetCameraTraceHit`))
    (`self.CreateMultiLineTrace` _outhit)
    (else
      (`KismetSystemLibrary.K2_ClearAndInvalidateTimerHandle` (`self.FullAutoTimer`))
      (`self.K2_EndAbility`))))

(fn `TraceDamage`
  (params (OutHits :type "Array of HitResult Structure"))
  (locals (LocalBottomCharacterSocketName :type Name :default "bottom_Socket") (LocalHitComponent :type "PrimitiveComponent Object Reference"))
  (for _array_element OutHits
    (bind (_bblockinghit _binitialoverlap _time _distance _location _impactpoint _normal _impactnormal _physmat _hitactor _hitcomponent) (`GameplayStatics.BreakHitResult` _array_element))
    (if (`KismetSystemLibrary.DoesImplementInterface` _hitactor "/Game/CombatSystem/Interfaces/BPI_CharacterIntreface.BPI_CharacterIntreface_C")
      (message `/Game/CombatSystem/Interfaces/BPI_CharacterIntreface.SetHitLocation` (`self.GetAvatarActorFromActorInfo`) _location)
      (set `self.DamagedActor` _hitactor)
      (set `local.LocalHitComponent` _hitcomponent)
      (if (`self.GetCanBeDamaged`)
        (bind _hitlocation (message `/Game/CombatSystem/Interfaces/BPI_CharacterIntreface.GetHitLocation` (`self.GetAvatarActorFromActorInfo`)))
        (bind _damagemultiplier (message `/Game/CombatSystem/Interfaces/BPI_CharacterIntreface.GetDamageMultiplier` (`self.GetAvatarActorFromActorInfo`)))
        (`self.ApplyDamage` (`self.DamagedActor`) (* (`/Game/CombatSystem/Weapons/BP_BaseWeapon.WeaponDamage` (`self.CurrentWeapon`)) (select `bool` (`KismetMathLibrary.InRange_FloatFloat` (.z (- _hitlocation (`SceneComponent.GetSocketLocation` (`local.LocalHitComponent`) (`local.LocalBottomCharacterSocketName`)))) 150.0 180.0) :`false` (`self.DefaultDamageMultiplier`) :`true` _damagemultiplier)))
        (set `self.LastHitActor` (`self.DamagedActor`)))))
  (return))

(fn `TraceDamageEndAbility`
  (set `self.LastHitActor` null)
  (`self.K2_EndAbility`))