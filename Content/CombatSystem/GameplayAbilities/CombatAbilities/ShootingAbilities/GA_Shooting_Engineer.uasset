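; Engineer shooting gameplay ability that fires a blast of randomly spread line traces from the weapon muzzle toward the aimed point.
; CreateMultiLineTrace takes the trace count from the avatar and passes hits to TraceDamage, which runs parent damage logic and commits cooldown.
; While the first Engineer ability is active, an alternate spread applies and shots are counted, clearing the ability at its limit.
; Firing also adds a CantFire tag.
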(event `self.K2_ActivateAbility`
  (`parent.K2_ActivateAbility`))

(event `self.K2_OnEndAbility`
  (params (bWasCancelled :type Boolean))
  (`parent.K2_OnEndAbility` bWasCancelled))

(fn `CreateMultiLineTrace`
  (params (Hit :type "HitResult Structure (by ref)"))
  (locals (LocalMinLineTraceSpread :type "Float (double-precision)" :default -750.0) (LocalMaxLineTraceSpread :type "Float (double-precision)" :default 750.0) (LocalMaxAmountOfShotsAbility :type Integer :default 5) (LocalDefaultValue :type Integer))
  (bind _returnvalue (`self.GetAvatarActorFromActorInfo`))
  (bind (_bblockinghit _binitialoverlap _time _distance _location _impactpoint _normal _impactnormal _physmat _hitactor _hitcomponent _hitbonename _bonename _hititem _elementindex _faceindex _tracestart _traceend) (`GameplayStatics.BreakHitResult` Hit))
  (bind _localminlinetracespread (`local.LocalMinLineTraceSpread`))
  (bind _localmaxlinetracespread (`local.LocalMaxLineTraceSpread`))
  (bind _returnvalue_2 (`SceneComponent.K2_GetComponentLocation` (`/Game/CombatSystem/Weapons/BP_BaseWeapon.Muzzle` (`self.CurrentWeapon`))))
  (bind _returnvalue_3 (select `bool` (`GameplayTagAssetInterface.HasMatchingGameplayTag` (`self.AbilitySystemComponent`) (struct :`TagName` "EngineerCharacter.Abilities.First.IsActive")) :`false` (`self.EngineerSpreadMultiplier`) :`true` (`self.AbilityEngineerSpreadMultiplier`)))
  (bind _returnvalue_4 (- _location _returnvalue_2))
  (bind _amountofshotsability (message `/Game/CombatSystem/Interfaces/BPI_EngineerCharacter.GetAmountOfShotsAbility` (`self.GetAvatarActorFromActorInfo`)))
  (if (and (>= _amountofshotsability (`local.LocalMaxAmountOfShotsAbility`)) (`GameplayTagAssetInterface.HasMatchingGameplayTag` (`self.AbilitySystemComponent`) (struct :`TagName` "EngineerCharacter.Abilities.First.IsActive")))
    (message `/Game/CombatSystem/Interfaces/BPI_EngineerCharacter.RemoveIsAbilityActiveTag` _returnvalue)
    (message `/Game/CombatSystem/Interfaces/BPI_EngineerCharacter.SetAmountOfShotsAbility` _returnvalue (`local.LocalDefaultValue`)))
  (bind _engineerblastamount (message `/Game/CombatSystem/Interfaces/BPI_EngineerCharacter.GetEngineerBlastAmount` (`self.GetAvatarActorFromActorInfo`)))
  (for _ (range (+ _engineerblastamount 1))
    (bind _outhits (`KismetSystemLibrary.LineTraceMulti` :`Start` _returnvalue_2 :`End` (+ (`KismetMathLibrary.SelectVector` (+ (* (/ _returnvalue_4 (`KismetMathLibrary.VSize` _returnvalue_4)) (`self.ShootingDistanceMultiplayer`)) _location) _traceend _bblockinghit) (`KismetMathLibrary.MakeVector` (* (`KismetMathLibrary.RandomFloatInRange` _localminlinetracespread _localmaxlinetracespread) _returnvalue_3) (* (`KismetMathLibrary.RandomFloatInRange` _localminlinetracespread _localmaxlinetracespread) _returnvalue_3) (* (`KismetMathLibrary.RandomFloatInRange` _localminlinetracespread _localmaxlinetracespread) _returnvalue_3))) :`TraceChannel` "TraceTypeQuery1" :`DrawDebugType` "ForDuration" :`bIgnoreSelf` false))
    (`self.TraceDamage` _outhits))
  (if (`GameplayTagAssetInterface.HasMatchingGameplayTag` (`self.AbilitySystemComponent`) (struct :`TagName` "EngineerCharacter.Abilities.First.IsActive"))
    (message `/Game/CombatSystem/Interfaces/BPI_EngineerCharacter.IncrementAmountOfShotsAbility` (`self.GetAvatarActorFromActorInfo`)))
  (if (not (`GameplayTagAssetInterface.HasMatchingGameplayTag` (`self.AbilitySystemComponent`) (struct :`TagName` "Character.States.CantFire")))
    (`AbilitySystemBlueprintLibrary.AddLooseGameplayTags` (`self.GetAvatarActorFromActorInfo`) (`BlueprintGameplayTagLibrary.MakeLiteralGameplayTagContainer` (struct :`GameplayTags` (struct :`(TagName` "Character.States.CantFire")))))))

(fn `GetLineTraceStartAndEnd`
  (params (Hit :type "HitResult Structure (by ref)"))
  (returns (StartLocation :type "Vector Structure") (EndLocation :type "Vector Structure"))
  (bind (_startlocation _endlocation) (`parent.GetLineTraceStartAndEnd` Hit))
  (return _startlocation _endlocation))

(fn `TraceDamage`
  (params (OutHits :type "Array of HitResult Structure (by ref)"))
  (`parent.TraceDamage` OutHits)
  (`self.K2_CommitAbilityCooldown` false)
  (return))