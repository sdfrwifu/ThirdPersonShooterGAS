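; GA_Shooting_AI is the AI variant of the shooting gameplay ability, overriding pieces of its parent's firing logic.
; Firing is allowed only when the current weapon has ammo and the owner has neither the reloading nor the can't-fire tag.
; The parent's line trace end gets a random per-axis spread offset to scatter shots.
; After the parent's trace damage runs, the ability force-commits its cooldown and ends.
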(fn `CanFireCheck`
  (returns (ReturnValue :type Boolean))
  (return (and (> (`/Game/CombatSystem/Weapons/BP_BaseWeapon.CurrentAmountOfAmmo` (`self.CurrentWeapon`)) 0.0) (not (`GameplayTagAssetInterface.HasMatchingGameplayTag` (`self.AbilitySystemComponent`) (struct :`TagName` "WeaponState.IsReloading"))) (not (`GameplayTagAssetInterface.HasMatchingGameplayTag` (`self.AbilitySystemComponent`) (struct :`TagName` "Character.States.CantFire"))))))

(fn `GetLineTraceStartAndEnd`
  (params (Hit :type "HitResult Structure (by ref)"))
  (returns (StartLocation :type "Vector Structure") (EndLocation :type "Vector Structure"))
  (locals (LocalMinLineTraceSpread :type "Float (double-precision)" :default -200.0) (LocalMaxLineTraceSpread :type "Float (double-precision)" :default 200.0))
  (bind (_startlocation _endlocation) (`parent.GetLineTraceStartAndEnd` Hit))
  (bind _localminlinetracespread (`local.LocalMinLineTraceSpread`))
  (bind _localmaxlinetracespread (`local.LocalMaxLineTraceSpread`))
  (return _startlocation (+ _endlocation (`KismetMathLibrary.MakeVector` (`KismetMathLibrary.RandomFloatInRange` _localminlinetracespread _localmaxlinetracespread) (`KismetMathLibrary.RandomFloatInRange` _localminlinetracespread _localmaxlinetracespread) (`KismetMathLibrary.RandomFloatInRange` _localminlinetracespread _localmaxlinetracespread)))))

(fn `TraceDamage`
  (params (OutHits :type "Array of HitResult Structure (by ref)"))
  (`parent.TraceDamage` OutHits)
  (`self.K2_CommitAbilityCooldown` false true)
  (`self.K2_EndAbility`)
  (return))