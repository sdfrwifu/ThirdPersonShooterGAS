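; Storm Trooper shooting ability that extends its parent's trace, damage and full-auto logic with hits-in-a-row ammo messages.
; Each damage trace commits the cooldown, then either clears a valid DamagedActor or sends the avatar the structure variant of that message.
; Applying damage sends the standard message.
; Clearing the full-auto timer adds a non-replicated CantFire loose tag if the avatar lacks it.
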(event `self.K2_ActivateAbility`
  (`parent.K2_ActivateAbility`))

(event `self.K2_OnEndAbility`
  (params (bWasCancelled :type Boolean))
  (`parent.K2_OnEndAbility` bWasCancelled))

(fn `ActivateTakeDamageFunction`
  (params (HitLocation :type "Vector Structure") (HitComponent :type "PrimitiveComponent Object Reference"))
  (`parent.ActivateTakeDamageFunction` HitLocation HitComponent)
  (message `/Game/CombatSystem/Interfaces/BPI_StormTrooperCharacter.AddHitsInRowAmmo` (`self.GetAvatarActorFromActorInfo`)))

(fn `ClearFullAutoTimer`
  (bind _returnvalue (`self.GetAvatarActorFromActorInfo`))
  (`parent.ClearFullAutoTimer`)
  (if (not (`GameplayTagAssetInterface.HasMatchingGameplayTag` (`Actor.GetComponentByClass` _returnvalue "/Script/TestProject.MyAbilitySystemComponent") (struct :`TagName` "Character.States.CantFire")))
    (`AbilitySystemBlueprintLibrary.AddLooseGameplayTags` _returnvalue (`BlueprintGameplayTagLibrary.MakeLiteralGameplayTagContainer` (struct :`GameplayTags` (struct :`(TagName` "Character.States.CantFire")))))))

(fn `TraceDamage`
  (params (OutHits :type "Array of HitResult Structure (by ref)"))
  (`parent.TraceDamage` OutHits)
  (`self.K2_CommitAbilityCooldown` false)
  (`/Engine/EditorBlueprintResources/StandardMacros.IsValid` (`self.DamagedActor`)
    (:`Is Valid`
      (set `self.DamagedActor` null))
    (:`Is Not Valid`
      (message `/Game/CombatSystem/Interfaces/BPI_StormTrooperCharacter.AddHitsInRowAmmoInStructure` (`self.GetAvatarActorFromActorInfo`))))
  (return))