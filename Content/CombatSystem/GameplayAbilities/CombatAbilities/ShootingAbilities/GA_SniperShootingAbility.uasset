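; Sniper shooting ability that extends a parent shooting ability with a cooldown and a damage-over-time effect for the sniper's first ability.
; After the parent trace, it applies a cooldown effect whose set-by-caller magnitude is the weapon's fire rate.
; If the first-ability tag is active, a looping timer deals tick damage until the maximum count, then clears the tag and ends.
; Otherwise, or without a valid hit actor, the ability ends.
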(event `self.K2_ActivateAbility`
  (`parent.K2_ActivateAbility`))

(event `self.K2_OnEndAbility`
  (params (bWasCancelled :type Boolean))
  (`parent.K2_OnEndAbility` bWasCancelled)
  (set `self.SniperAbilityAmountOfTicks` 0))

(event `SniperFirstAbility`
  (bind _returnvalue (`KismetSystemLibrary.K2_SetTimerDelegate` (delegate `SniperAbilityDamageEvent`) (`self.SniperAbilityTickTimeRate`) true))
  (set `self.SniperAbilityTimer` _returnvalue))

(event `SniperAbilityDamageEvent`
  (`self.SniperFirstAbilityDamage`))

(fn `SniperFirstAbilityDamage`
  (locals (LocalSniperAbilityTickDamage :type "Float (double-precision)" :default 5.0))
  (`GameplayStatics.ApplyDamage` (`self.DamagedActor`) (`local.LocalSniperAbilityTickDamage`))
  (bind _result (`/Engine/EditorBlueprintResources/StandardMacros.IncrementInt` (`self.SniperAbilityAmountOfTicks`))
    (:`  `
      (if (== _result (`self.SniperMaxAmountOfTicks`))
        (`KismetSystemLibrary.K2_ClearAndInvalidateTimerHandle` (`self.SniperAbilityTimer`))
        (`AbilitySystemBlueprintLibrary.RemoveLooseGameplayTags` (`self.GetAvatarActorFromActorInfo`) (`BlueprintGameplayTagLibrary.MakeLiteralGameplayTagContainer` (struct :`GameplayTags` (struct :`(TagName` "SniperCharacter.Abilities.First.IsActive")))))
        (`self.K2_EndAbility`)))))

(fn `TraceDamage`
  (params (OutHits :type "Array of HitResult Structure (by ref)"))
  (locals (LocalHitComponent :type "PrimitiveComponent Object Reference") (LocalBottomCharacterSocketName :type Name :default "bottom_Socket"))
  (`parent.TraceDamage` OutHits)
  (if (not (`GameplayTagAssetInterface.HasMatchingGameplayTag` (`self.AbilitySystemComponent`) (struct :`TagName` "SniperCharacter.Abilities.Shooting.Cooldown")))
    (bind _returnvalue (`AbilitySystemBlueprintLibrary.AssignTagSetByCallerMagnitude` (`self.MakeOutgoingGameplayEffectSpec` (`self.AbilityGameplayEffectCooldown`)) (struct :`TagName` "SniperCharacter.Abilities.Shooting.Data") (`/Game/CombatSystem/Weapons/BP_BaseWeapon.WeaponFireRate` (`self.CurrentWeapon`))))
    (`self.K2_ApplyGameplayEffectSpecToOwner` _returnvalue))
  (if (`GameplayTagAssetInterface.HasMatchingGameplayTag` (`self.AbilitySystemComponent`) (struct :`TagName` "SniperCharacter.Abilities.First.IsActive"))
    (`self.SniperFirstAbility`)
    (else
      (set `self.LastHitActor` null)
      (`self.K2_EndAbility`))))

(fn `TraceDamageEndAbility`
  (`self.LastHitActor`
    (:`then`)
    (:`else`
      (`self.K2_EndAbility`)
      (return))))