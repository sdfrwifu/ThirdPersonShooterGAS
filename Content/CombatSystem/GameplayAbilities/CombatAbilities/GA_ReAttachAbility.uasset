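; Gameplay ability that slides the character's current weapon between idle and jogging right-hand sockets based on movement speed.
; Unless a grenade throw is active, activation sets the IsJogging tag, snapshots both socket transforms and ends if the weapon already matches the target.
; Otherwise a looping timer, guarded by an IsAttaching tag, steps an alpha stored on the avatar and lerps the weapon transform until either limit ends the ability.
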(event `self.K2_ActivateAbility`
  (bind _returnvalue (`BlueprintGameplayTagLibrary.MakeLiteralGameplayTagContainer` (struct :`GameplayTags` (struct :`(TagName` "Character.States.IsJogging")))))
  (bind _returnvalue_2 (`self.GetAvatarActorFromActorInfo`))
  (bind _returnvalue_3 (`self.GetAvatarActorFromActorInfo`))
  (bind _righthandweaponjogsocket (`self.RightHandWeaponJogSocket`))
  (bind _righthandweaponsocket (`self.RightHandWeaponSocket`))
  (set `self.AbilitySystemComponent` (`Actor.GetComponentByClass` (`self.GetAvatarActorFromActorInfo`) "/Script/TestProject.MyAbilitySystemComponent"))
  (if (not (`GameplayTagAssetInterface.HasMatchingGameplayTag` (`self.AbilitySystemComponent`) (struct :`TagName` "Character.StormTrooper.States.IsGrenadeThrow")))
    (bind _abp_manny (message `/Game/CombatSystem/Interfaces/BPI_CharacterIntreface.GetCharacterABP` _returnvalue_3))
    (if (>= (`KismetMathLibrary.VSize` (`Actor.GetVelocity` _returnvalue_3)) (`/Game/CombatSystem/Animations/ABP_Manny.CharacterWalkSpeed` _abp_manny))
      (`AbilitySystemBlueprintLibrary.AddLooseGameplayTags` _returnvalue_2 _returnvalue)
      (else
        (`AbilitySystemBlueprintLibrary.RemoveLooseGameplayTags` _returnvalue_2 _returnvalue)))
    (bind (_righthandweaponsocket_2 _righthandweaponjogsocket_2) (message `/Game/CombatSystem/Interfaces/BPI_CharacterIntreface.GetCharacterHandSockets` (`self.GetAvatarActorFromActorInfo`)))
    (set `self.JoggingWeaponLocation` (`SceneComponent.GetSocketLocation` _righthandweaponjogsocket_2 _righthandweaponjogsocket))
    (set `self.JoggindWeaponRotation` (`SceneComponent.GetSocketRotation` _righthandweaponjogsocket_2 _righthandweaponjogsocket))
    (bind _righthandweaponsocket_3 (message `/Game/CombatSystem/Interfaces/BPI_CharacterIntreface.GetCharacterHandSockets` (`self.GetAvatarActorFromActorInfo`)))
    (set `self.IdleWeaponLocation` (`SceneComponent.GetSocketLocation` _righthandweaponsocket_3 _righthandweaponsocket))
    (set `self.IdleWeaponRoatation` (`SceneComponent.GetSocketRotation` _righthandweaponsocket_3 _righthandweaponsocket))
    (if (`GameplayTagAssetInterface.HasMatchingGameplayTag` (`self.AbilitySystemComponent`) (struct :`TagName` "Character.States.IsJogging"))
      (bind (_mainweapon _secondweapon _currentweapon) (message `/Game/CombatSystem/Interfaces/BPI_CharacterIntreface.GetCharacterWeapons` (`self.GetAvatarActorFromActorInfo`)))
      (if (and (== (`Actor.K2_GetActorLocation` _currentweapon) (`self.JoggingWeaponLocation`)) (== (`Actor.K2_GetActorRotation` _currentweapon) (`self.JoggindWeaponRotation`)))
        (`self.K2_EndAbility`)
        (else
          (if (not (`GameplayTagAssetInterface.HasMatchingGameplayTag` (`self.AbilitySystemComponent`) (struct :`TagName` "Character.States.IsAttaching"))) :!label _label
            (`AbilitySystemBlueprintLibrary.AddLooseGameplayTags` (`self.GetAvatarActorFromActorInfo`) (`BlueprintGameplayTagLibrary.MakeLiteralGameplayTagContainer` (struct :`GameplayTags` (struct :`(TagName` "Character.States.IsAttaching")))))
            (bind _returnvalue_4 (`KismetSystemLibrary.K2_SetTimerDelegate` (delegate `WeaponReAttach`) (`self.AttachLerpTickTimeRate`) true))
            (set `self.AttachTimer` _returnvalue_4))))
      (else
        (bind (_mainweapon_2 _secondweapon_2 _currentweapon_2) (message `/Game/CombatSystem/Interfaces/BPI_CharacterIntreface.GetCharacterWeapons` (`self.GetAvatarActorFromActorInfo`)))
        (if (and (== (`Actor.K2_GetActorRotation` _currentweapon_2) (`self.IdleWeaponRoatation`)) (== (`Actor.K2_GetActorLocation` _currentweapon_2) (`self.IdleWeaponLocation`)))
          (`self.K2_EndAbility`)
          (else
            (goto _label)))))))

(event `WeaponReAttach`
  (`self.WeaponReAttachChange` (* (`self.AttachLerpChangeRate`) (`KismetMathLibrary.SelectFloat` 1.0 -1.0 (`GameplayTagAssetInterface.HasMatchingGameplayTag` (`self.AbilitySystemComponent`) (struct :`TagName` "Character.States.IsJogging"))))))

(event `self.K2_OnEndAbility`
  (params (bWasCancelled :type Boolean)))

(fn `WeaponReAttachChange`
  (params (AttachLerpChangeRate :type "Float (double-precision)"))
  (locals (LocalMinAlphaValue :type "Float (double-precision)") (LocalMaxAlphaValue :type "Float (double-precision)" :default 1.0) (LocalAttachLerpEnd :type "Float (double-precision)" :default 1.0) (LocalAttachLerpEndWalk :type "Float (double-precision)"))
  (bind _returnvalue (`self.GetAvatarActorFromActorInfo`))
  (bind _returnvalue_2 (`self.GetAvatarActorFromActorInfo`))
  (bind _attachalpha (message `/Game/CombatSystem/Interfaces/BPI_CharacterIntreface.GetAttachAlpha` _returnvalue_2))
  (message `/Game/CombatSystem/Interfaces/BPI_CharacterIntreface.SetAttachAlpha` _returnvalue_2 (+ (`KismetMathLibrary.FClamp` _attachalpha (`local.LocalMinAlphaValue`) (`local.LocalMaxAlphaValue`)) AttachLerpChangeRate))
  (bind (_mainweapon _secondweapon _currentweapon) (message `/Game/CombatSystem/Interfaces/BPI_CharacterIntreface.GetCharacterWeapons` _returnvalue))
  (bind _attachalpha_2 (message `/Game/CombatSystem/Interfaces/BPI_CharacterIntreface.GetAttachAlpha` _returnvalue))
  (`Actor.K2_SetActorLocationAndRotation` _currentweapon (`KismetMathLibrary.VLerp` (`self.IdleWeaponLocation`) (`self.JoggingWeaponLocation`) _attachalpha_2) (`KismetMathLibrary.RLerp` (`self.IdleWeaponRoatation`) (`self.JoggindWeaponRotation`) _attachalpha_2 true) false false)
  (if (>= _attachalpha_2 (`local.LocalAttachLerpEnd`))
    (`AbilitySystemBlueprintLibrary.RemoveLooseGameplayTags` (`self.GetAvatarActorFromActorInfo`) (`BlueprintGameplayTagLibrary.MakeLiteralGameplayTagContainer` (struct :`GameplayTags` (struct :`(TagName` "Character.States.IsAttaching")))) :!label _label)
    (`KismetSystemLibrary.K2_ClearAndInvalidateTimerHandle` (`self.AttachTimer`))
    (`self.K2_EndAbility`)
    (elif (<= _attachalpha_2 (`local.LocalAttachLerpEndWalk`))
      (goto _label))))