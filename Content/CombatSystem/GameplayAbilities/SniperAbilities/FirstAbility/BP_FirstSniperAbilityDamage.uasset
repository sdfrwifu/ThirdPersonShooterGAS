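; Looping gameplay cue notify that deals the Sniper first ability's damage over time to its target.
; On looping start, a repeating timer runs SniperFirstAbilityDamage each tick.
; Each tick calls ApplyDamage, then subtracts the returned amount from the target's health through message calls.
; At the maximum tick count, it clears the timer and removes active effects granting the Character.States.SniperFirstAbilityDamage tag from the target's ability system component.
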(event `self.OnLoopingStart`
  (params (Target :type "Actor Object Reference") (Parameters :type "GameplayCueParameters Structure (by ref)") (SpawnResults :type "GameplayCueNotify_SpawnResult Structure (by ref)"))
  (bind _returnvalue (`KismetSystemLibrary.K2_SetTimerDelegate` (delegate `SniperAbilityDamageEvent`) (`self.SniperAbilityTickTimeRate`) true))
  (set `self.SniperAbilityTimer` _returnvalue))

(event `SniperAbilityDamageEvent`
  (`self.SniperFirstAbilityDamage` (stale `self.OnLoopingStart` Target)))

(fn `SniperFirstAbilityDamage`
  (params (DamagedActor :type "Actor Object Reference"))
  (locals (LocalSniperAbilityTickDamage :type "Float (double-precision)" :default 5.0) (LocalSniperMaxAmountOfTicks :type Integer :default 4))
  (bind _returnvalue (`GameplayStatics.ApplyDamage` DamagedActor (`local.LocalSniperAbilityTickDamage`)))
  (bind _currenthealth (message `/Game/CombatSystem/Interfaces/BPI_BaseCharacter.GetCharacterHealth` DamagedActor))
  (message `/Game/CombatSystem/Interfaces/BPI_BaseCharacter.SetCurrentHealth` DamagedActor (- _currenthealth _returnvalue))
  (bind _result (`/Engine/EditorBlueprintResources/StandardMacros.IncrementInt` (`self.SniperAbilityAmountOfTicks`))
    (:`  `
      (if (== _result (`local.LocalSniperMaxAmountOfTicks`))
        (`KismetSystemLibrary.K2_ClearAndInvalidateTimerHandle` null (`self.SniperAbilityTimer`))
        (`AbilitySystemComponent.RemoveActiveEffectsWithGrantedTags` (`self.GetComponentByClass` DamagedActor "/Script/TestProject.MyAbilitySystemComponent") (struct :`GameplayTags` (struct :`(TagName` "Character.States.SniperFirstAbilityDamage"))))))))

(fn `UserConstructionScript`)