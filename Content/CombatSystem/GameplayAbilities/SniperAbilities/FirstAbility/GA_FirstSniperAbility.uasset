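; GA_FirstSniperAbility is the sniper character's first gameplay ability, applying damage over time to a target actor.
; Activation commits the ability, starts a looping tick timer and forces the cooldown.
; Each tick applies damage to the stored DamagedActor, which is not assigned in this graph.
; At the maximum tick count it resets the counter, clears the timer, removes the owner's active-state effect by tag and ends the ability.
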(event `self.K2_ActivateAbility`
  (`self.K2_CommitAbility`)
  (cast `/Game/CombatSystem/Characters/BP_BaseThirdPersonCharacter` (`self.GetAvatarActorFromActorInfo`))
  (bind _returnvalue (`KismetSystemLibrary.K2_SetTimerDelegate` (delegate `SniperAbilityDamageEvent`) (`self.SniperAbilityTickTimeRate`) true))
  (set `self.SniperAbilityTimer` _returnvalue)
  (`self.K2_CommitAbilityCooldown` false true))

(event `SniperAbilityDamageEvent`
  (`self.SniperAbilityDamage` (`self.DamagedActor`)))

(fn `SniperAbilityDamage`
  (params (DamagedActor :type "Actor Object Reference"))
  (locals (LocalSniperAbilityTickDamage :type "Float (double-precision)" :default 5.0) (LocalMaxAmountOfTicks :type Integer :default 4))
  (`GameplayStatics.ApplyDamage` DamagedActor (`local.LocalSniperAbilityTickDamage`))
  (bind _result (`/Engine/EditorBlueprintResources/StandardMacros.IncrementInt` (`self.AbilityAmountOfTicks`))
    (:`  `
      (if (== _result (`local.LocalMaxAmountOfTicks`))
        (set `self.AbilityAmountOfTicks` 0)
        (`KismetSystemLibrary.K2_ClearAndInvalidateTimerHandle` (`self.SniperAbilityTimer`))
        (`self.BP_RemoveGameplayEffectFromOwnerWithGrantedTags` (struct :`GameplayTags` (struct :`(TagName` "SniperCharacter.Abilities.First.IsActive"))))
        (`self.K2_EndAbility`)))))