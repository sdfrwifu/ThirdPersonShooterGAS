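; Sniper's second gameplay ability, which toggles between the main weapon and the pistol.
; A loose IsCurrentWeaponPistol tag tracks the state, while message calls on the avatar move the weapons between back and right-hand sockets.
; Each swap clears aiming, updates walk speed (never below default), refills the new weapon's clip and refreshes the widget text.
; The ability ends when the equip montage completes or is interrupted.
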(event `self.K2_ActivateAbility`
  (bind _returnvalue (`self.GetAvatarActorFromActorInfo`))
  (bind _returnvalue_2 (`self.GetAvatarActorFromActorInfo`))
  (bind _returnvalue_3 (`self.GetAvatarActorFromActorInfo`))
  (bind _returnvalue_4 (`self.GetAvatarActorFromActorInfo`))
  (bind _returnvalue_5 (`BlueprintGameplayTagLibrary.MakeLiteralGameplayTagContainer` (struct :`GameplayTags` (struct :`(TagName` "Character.Sniper.States.IsCurrentWeaponPistol")))))
  (`self.K2_CommitAbility`)
  (if (`GameplayTagAssetInterface.HasMatchingGameplayTag` (`Actor.GetComponentByClass` (`self.GetAvatarActorFromActorInfo`) "/Script/TestProject.MyAbilitySystemComponent") (struct :`TagName` "Character.Sniper.States.IsCurrentWeaponPistol"))
    (`AbilitySystemBlueprintLibrary.RemoveLooseGameplayTags` _returnvalue_4 _returnvalue_5)
    (bind (_mainweapon _secondweapon) (message `/Game/CombatSystem/Interfaces/BPI_BaseCharacter.GetCharacterWeapons` _returnvalue))
    (message `/Game/CombatSystem/Interfaces/BPI_SniperCharacter.SetCurrentWeapon` _returnvalue _mainweapon)
    (message `/Game/CombatSystem/Interfaces/BPI_BaseCharacter.CallAttachWeapon` _returnvalue _secondweapon (`self.BackWeaponSocket`))
    (else
      (`AbilitySystemBlueprintLibrary.AddLooseGameplayTags` _returnvalue_4 _returnvalue_5)
      (bind (_mainweapon_2 _secondweapon_2) (message `/Game/CombatSystem/Interfaces/BPI_BaseCharacter.GetCharacterWeapons` _returnvalue_2))
      (message `/Game/CombatSystem/Interfaces/BPI_SniperCharacter.SetCurrentWeapon` _returnvalue_2 _secondweapon_2)
      (message `/Game/CombatSystem/Interfaces/BPI_BaseCharacter.CallAttachWeapon` _returnvalue_2 _mainweapon_2 (`self.BackWeaponSocket`))))
  (bind (_mainweapon_3 _secondweapon_3 _currentweapon) (message `/Game/CombatSystem/Interfaces/BPI_BaseCharacter.GetCharacterWeapons` _returnvalue_3))
  (message `/Game/CombatSystem/Interfaces/BPI_BaseCharacter.CallAttachWeapon` _returnvalue_3 _currentweapon (`self.RightHandWeaponSocketName`))
  (`self.NotAimingSettings`)
  (bind (_mainweapon_4 _secondweapon_4 _currentweapon_2) (message `/Game/CombatSystem/Interfaces/BPI_BaseCharacter.GetCharacterWeapons` (`self.GetAvatarActorFromActorInfo`)))
  (message `/Game/CombatSystem/Interfaces/BPI_Weapon.SetCurrentAmmo` _currentweapon_2 (`/Game/CombatSystem/Weapons/BP_BaseWeapon.ClipAmount` _currentweapon_2))
  (`self.SetTextToWidget`)
  (`AbilityTask_PlayMontageAndWait.CreatePlayMontageAndWaitProxy` "None" "/Game/CombatSystem/Animations/AM_MM_Rifle_Equip.AM_MM_Rifle_Equip"
    (:`OnCompleted`
      _)
    (:`OnInterrupted`
      _))
  (`self.K2_EndAbility`))

(fn `NotAimingSettings`
  (if (`GameplayTagAssetInterface.HasMatchingGameplayTag` (`Actor.GetComponentByClass` (`self.GetAvatarActorFromActorInfo`) "/Script/TestProject.MyAbilitySystemComponent") (struct :`TagName` "Character.States.IsAiming"))
    (`AbilitySystemBlueprintLibrary.RemoveLooseGameplayTags` (`self.GetAvatarActorFromActorInfo`) (`BlueprintGameplayTagLibrary.MakeLiteralGameplayTagContainer` (struct :`GameplayTags` (struct :`(TagName` "Character.States.IsAiming"))))))
  (message `/Game/CombatSystem/Interfaces/BPI_BaseCharacter.SetCurrentMaxCharacterSpeed` (`self.GetAvatarActorFromActorInfo`) (`KismetMathLibrary.SelectFloat` (`self.MaxPistolCharacterSpeed`) (`self.MaxDefaultCharacterSpeed`) (`GameplayTagAssetInterface.HasMatchingGameplayTag` (`Actor.GetComponentByClass` (`self.GetAvatarActorFromActorInfo`) "/Script/TestProject.MyAbilitySystemComponent") (struct :`TagName` "Character.Sniper.States.IsCurrentWeaponPistol"))))
  (bind _currentmaxspeed (message `/Game/CombatSystem/Interfaces/BPI_BaseCharacter.GetCurrentMaxCharacterSpeed` (`self.GetAvatarActorFromActorInfo`)))
  (set `CharacterMovementComponent.MaxWalkSpeed` (`KismetMathLibrary.SelectFloat` _currentmaxspeed (`self.MaxDefaultCharacterSpeed`) (> _currentmaxspeed (`self.MaxDefaultCharacterSpeed`))) (`Actor.GetComponentByClass` (`self.GetAvatarActorFromActorInfo`) "/Script/Engine.CharacterMovementComponent")))