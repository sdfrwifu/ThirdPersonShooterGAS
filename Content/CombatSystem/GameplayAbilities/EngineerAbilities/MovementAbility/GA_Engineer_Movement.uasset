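; Engineer movement gameplay ability that temporarily boosts the avatar's walk speed and jump height.
; On activation it commits, then multiplies the CharacterMovementComponent's MaxWalkSpeed and JumpZVelocity, ending at once if no component is found.
; A WaitDelay task times the boost, then divides the current values by the same multipliers and ends the ability.
; The revert runs only when that delay finishes, with no handling for early cancellation.
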(event `self.K2_ActivateAbility`
  (bind _movementcomponent (`self.MovementComponent`))
  (bind _returnvalue (`Actor.GetComponentByClass` (`self.GetAvatarActorFromActorInfo`) "/Script/Engine.CharacterMovementComponent"))
  (`self.K2_CommitAbility`)
  (`/Engine/EditorBlueprintResources/StandardMacros.IsValid` _returnvalue
    (:`Is Valid`
      (bind _output_get (set `self.MovementComponent` _returnvalue))
      (bind _output_get_2 (set `self.StartMaxCharacterSpeed` (`CharacterMovementComponent.MaxWalkSpeed` _output_get)))
      (set `CharacterMovementComponent.MaxWalkSpeed` (* _output_get_2 (`self.WalkSpeedMultiplier`)) (`self.MovementComponent`))
      (bind _output_get_3 (set `self.StartJumpZVelocity` (`CharacterMovementComponent.JumpZVelocity` (`self.MovementComponent`))))
      (set `CharacterMovementComponent.JumpZVelocity` (* _output_get_3 (`self.AbilityJumpMultiplier`)) (`self.MovementComponent`))
      (`AbilityTask_WaitDelay.WaitDelay` (`self.AbilityDuration`)
        (:`OnFinish`
          (set `CharacterMovementComponent.MaxWalkSpeed` (/ (`CharacterMovementComponent.MaxWalkSpeed` (`self.MovementComponent`)) (`self.WalkSpeedMultiplier`)) _movementcomponent)
          (set `CharacterMovementComponent.JumpZVelocity` (/ (`CharacterMovementComponent.JumpZVelocity` _movementcomponent) (`self.AbilityJumpMultiplier`)) (`self.MovementComponent`))
          (`self.K2_EndAbility`))))
    (:`Is Not Valid`
      (`self.K2_EndAbility`))))