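; Gameplay ability for the Engineer's drone that locks it onto an enemy character as its current target.
; On activation, if no target is held and the drone is not dead, it stores the enemy and starts a looping rotation timer.
; It then issues an AI move to the enemy's location at activation and sets the floating movement's lock-on max speed.
; The rotation event and the rotate and color-change functions are empty here.
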(event `self.K2_ActivateAbility`
  (bind _asbp_enemy_third_person_character (cast `/Game/CombatSystem/Characters/BP_EnemyThirdPersonCharacter` null))
  (if (and (not (`KismetSystemLibrary.IsValid` (`self.CurrentTarget`))) (not (`GameplayTagAssetInterface.HasMatchingGameplayTag` (`Actor.GetComponentByClass` (`self.GetAvatarActorFromActorInfo`) "/Script/TestProject.MyAbilitySystemComponent") (struct :`TagName` "Character.States.IsDead"))))
    (set `self.CurrentTarget` _asbp_enemy_third_person_character)
    (bind _returnvalue (`KismetSystemLibrary.K2_SetTimerDelegate` (delegate `RotatingLerp`) (`self.RotateLerpTickTimeRate`) true))
    (set `self.RotateLerpTimer` _returnvalue)
    (`AITask_MoveTo.AIMoveTo` (`AIBlueprintHelperLibrary.GetAIController` (`self.GetAvatarActorFromActorInfo`)) (`Actor.K2_GetActorLocation` _asbp_enemy_third_person_character) null 25.0 "Disable" "Default" false
      (:`then`
        (set `FloatingPawnMovement.MaxSpeed` (`self.MaxDroneLockOnTargetSpeed`) (`self.FloatingPawnMovement`))))))

(event `RotatingLerp`)