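; GA_Engineer_Second is the Engineer's second gameplay ability, which deploys a drone pawn in front of the avatar.
; On activation it line-traces on the Camera channel along the avatar's forward vector and compares the hit distance to the spawn distance.
; If the distance is greater, it spawns the drone at that offset, owned by the avatar, then commits and ends.
; Otherwise it ends without committing.
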(event `self.K2_ActivateAbility`
  (bind _returnvalue (`self.GetAvatarActorFromActorInfo`))
  (bind _returnvalue_2 (`self.GetAvatarActorFromActorInfo`))
  (bind _returnvalue_3 (`Actor.K2_GetActorLocation` _returnvalue_2))
  (bind _outhit (`KismetSystemLibrary.LineTraceSingle` :`Start` _returnvalue_3 :`End` (+ _returnvalue_3 (* (`Actor.GetActorForwardVector` _returnvalue_2) (`self.CameraTraceDistance`))) :`TraceChannel` "TraceTypeQuery2" :`TraceColor` (struct :`R` 1.0 :`B` 0.826939 :`A` 1.0)))
  (if (> (`.Distance` (`GameplayStatics.BreakHitResult` _outhit)) (`self.DroneSpawnDistance`))
    (`|SpawnActorFromClass` "/Game/CombatSystem/Drone/DronePawn.DronePawn_C" (`KismetMathLibrary.MakeTransform` (+ (* (`Actor.GetActorForwardVector` _returnvalue) (`self.DroneSpawnDistance`)) (`Actor.K2_GetActorLocation` _returnvalue)) (`Actor.K2_GetActorRotation` _returnvalue)) "AlwaysSpawn" "MultiplyWithRoot" _returnvalue (`GameplayStatics.GetPlayerPawn` 0))
    (`self.K2_CommitAbility`)
    (`self.K2_EndAbility`)
    (else
      (`self.K2_EndAbility`))))