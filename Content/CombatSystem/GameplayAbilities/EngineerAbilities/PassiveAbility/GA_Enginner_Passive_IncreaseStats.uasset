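; Engineer passive gameplay ability that boosts the character's stats for being in the drone aura.
; On activation it adds a non-replicated IsInDroneAura loose tag to the avatar if absent.
; It then multiplies movement speed and increases the shooting component's blast amount, whether or not the tag was already present.
; The ability neither reverts these changes nor ends itself.
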(event `self.K2_ActivateAbility`
  (bind _returnvalue (`Actor.GetComponentByClass` (`self.GetAvatarActorFromActorInfo`) "/Script/Engine.CharacterMovementComponent"))
  (bind _shootingcomponent (`/Game/CombatSystem/Characters/BP_BaseThirdPersonCharacter.ShootingComponent` (`self.BP_EngineerThirdPersonCharacter`)))
  (if (not (`GameplayTagAssetInterface.HasMatchingGameplayTag` (`Actor.GetComponentByClass` (`self.GetAvatarActorFromActorInfo`) "/Script/TestProject.MyAbilitySystemComponent") (struct :`TagName` "Character.Engineer.States.IsInDroneAura")))
    (`AbilitySystemBlueprintLibrary.AddLooseGameplayTags` (`self.GetAvatarActorFromActorInfo`) (`BlueprintGameplayTagLibrary.MakeLiteralGameplayTagContainer` (struct :`GameplayTags` (struct :`(TagName` "Character.Engineer.States.IsInDroneAura"))))))
  (set `CharacterMovementComponent.MaxWalkSpeed` (* (`MovementComponent.GetMaxSpeed` _returnvalue) (`self.SpeedMultiplierInDroneAura`)) _returnvalue)
  (set `/Game/CombatSystem/Components/BP_BaseShootingComponent.EnginnerBlastAmount` (+ (`/Game/CombatSystem/Components/BP_BaseShootingComponent.EnginnerBlastAmount` _shootingcomponent) (`self.BlastAmountInreaseInDroneAura`)) _shootingcomponent))