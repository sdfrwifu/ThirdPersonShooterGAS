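; Engineer passive gameplay ability that reverts the stat bonuses granted by the drone aura.
; On activation it commits, removes the IsInDroneAura loose tag from the avatar if present, then divides max walk speed by the aura speed multiplier and subtracts the aura's blast amount increase before ending.
; The stat reversal runs regardless of whether the tag was present, and speed is derived from the current max speed rather than a stored base.
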(event `self.K2_ActivateAbility`
  (bind _returnvalue (`self.GetAvatarActorFromActorInfo`))
  (bind _returnvalue_2 (`Actor.GetComponentByClass` (`self.GetAvatarActorFromActorInfo`) "/Script/Engine.CharacterMovementComponent"))
  (`self.K2_CommitAbility`)
  (if (`GameplayTagAssetInterface.HasMatchingGameplayTag` (`Actor.GetComponentByClass` (`self.GetAvatarActorFromActorInfo`) "/Script/TestProject.MyAbilitySystemComponent") (struct :`TagName` "Character.Engineer.States.IsInDroneAura"))
    (`AbilitySystemBlueprintLibrary.RemoveLooseGameplayTags` (`self.GetAvatarActorFromActorInfo`) (`BlueprintGameplayTagLibrary.MakeLiteralGameplayTagContainer` (struct :`GameplayTags` (struct :`(TagName` "Character.Engineer.States.IsInDroneAura"))))))
  (set `CharacterMovementComponent.MaxWalkSpeed` (/ (`MovementComponent.GetMaxSpeed` _returnvalue_2) (`self.SpeedMultiplierInDroneAura`)) _returnvalue_2)
  (bind _engineerblastamount (message `/Game/CombatSystem/Interfaces/BPI_EngineerCharacter.GetEngineerBlastAmount` _returnvalue))
  (message `/Game/CombatSystem/Interfaces/BPI_EngineerCharacter.SetEngineerBlastAmount` _returnvalue (- _engineerblastamount (`self.BlastAmountInreaseInDroneAura`)))
  (`self.K2_EndAbility`))