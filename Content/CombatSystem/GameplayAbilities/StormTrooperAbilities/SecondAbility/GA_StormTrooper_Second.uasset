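; StormTrooper's second gameplay ability, which throws a grenade using a rifle grenade-toss montage.
; On montage blend out, it reattaches the current weapon to the right-hand socket and line traces forward from the character's camera.
; It spawns BP_Grenade at the left hand, aimed at the trace hit or along camera rotation on a miss, then passes it to the avatar.
; Montage completion, interruption or cancellation ends the ability.
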(event `self.K2_ActivateAbility`
  (bind _returnvalue (`self.GetAvatarActorFromActorInfo`))
  (bind _returnvalue_2 (`SceneComponent.GetSocketLocation` (`Actor.GetComponentByClass` (`self.GetAvatarActorFromActorInfo`) "/Script/Engine.SkeletalMeshComponent") "hand_l"))
  (`AbilityTask_PlayMontageAndWait.CreatePlayMontageAndWaitProxy` "None" "/Game/CombatSystem/Animations/AM_MM_Rifle_GrenadeToss.AM_MM_Rifle_GrenadeToss"
    (:`OnCompleted`
      (`self.K2_EndAbility` :!label _label))
    (:`OnBlendOut`
      (bind (_mainweapon _secondweapon _currentweapon) (message `/Game/CombatSystem/Interfaces/BPI_BaseCharacter.GetCharacterWeapons` _returnvalue))
      (message `/Game/CombatSystem/Interfaces/BPI_BaseCharacter.CallAttachWeapon` _returnvalue _currentweapon "RightHandWeaponSocket")
      (bind _cameracomponent (message `/Game/CombatSystem/Interfaces/BPI_BaseCharacter.GetCharacterCamera` (`self.GetAvatarActorFromActorInfo`)))
      (bind _returnvalue_3 (`SceneComponent.K2_GetComponentLocation` _cameracomponent))
      (bind _outhit (`KismetSystemLibrary.LineTraceSingle` :`Start` _returnvalue_3 :`End` (+ _returnvalue_3 (* (`SceneComponent.GetForwardVector` _cameracomponent) (`self.ShootingDistanceMultiplayer`))) :`TraceChannel` "TraceTypeQuery2" :`TraceColor` (struct :`R` 1.0 :`B` 0.826939 :`A` 1.0)))
      (bind (_bblockinghit _binitialoverlap _time _distance _location) (`GameplayStatics.BreakHitResult` _outhit))
      (bind _returnvalue_4 (`|SpawnActorFromClass` "/Game/CombatSystem/Weapons/Grenade/BP_Grenade.BP_Grenade_C" (`KismetMathLibrary.MakeTransform` _returnvalue_2 (`KismetMathLibrary.SelectRotator` (`KismetMathLibrary.Conv_VectorToRotator` (`KismetMathLibrary.GetDirectionUnitVector` _returnvalue_2 _location)) (`Actor.K2_GetActorRotation` (`GameplayStatics.GetPlayerCameraManager` 0)) _bblockinghit)) "AlwaysSpawn" "MultiplyWithRoot" (`self.GetAvatarActorFromActorInfo`) null))
      (message `/Game/CombatSystem/Interfaces/BPI_StormTrooperCharacter.SetGrenadeBlueprint` (`self.GetAvatarActorFromActorInfo`) _returnvalue_4))
    (:`OnInterrupted`
      (goto _label))
    (:`OnCancelled`
      (goto _label))))