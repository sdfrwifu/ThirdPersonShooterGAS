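; Stormtrooper gameplay ability intended for aiming a grenade throw with trajectory prediction, currently inactive because ActivateAbility is empty.
; Its disconnected graph attaches the current weapon to the back socket and chains two grenade-toss montages before ending the ability.
; As the second montage starts, it runs a single projectile-path prediction from the left hand along camera forward, ignoring avatar and weapon, without using the result.
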(event `self.K2_ActivateAbility`)