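; Gameplay ability that deals the StormTrooper grenade's area damage to characters caught in its hit results.
; On activation it gets the hit results and grenade from the avatar through message calls, filtering for BPI_BaseCharacter implementers.
; Damage falls off linearly with distance over the grenade's sphere radius, clamped between minimum and maximum, and goes through ApplyDamage.
; LastHitActor skips only consecutive duplicate hits and clears when the ability ends.
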(event `self.K2_ActivateAbility`
  (bind _hitresults (message `/Game/CombatSystem/Interfaces/BPI_StormTrooperCharacter.GetGrenadeHitResults` (`self.GetAvatarActorFromActorInfo`)))
  (for _array_element _hitresults
    (bind _granadeblueprint (message `/Game/CombatSystem/Interfaces/BPI_StormTrooperCharacter.GetGrenadeBlueprint` (`self.GetAvatarActorFromActorInfo`)))
    (bind (_bblockinghit _binitialoverlap _time _distance _location _impactpoint _normal _impactnormal _physmat _hitactor) (`GameplayStatics.BreakHitResult` _array_element))
    (if (and (`KismetSystemLibrary.DoesImplementInterface` _hitactor "/Game/CombatSystem/Interfaces/BPI_BaseCharacter.BPI_BaseCharacter_C") (!= _hitactor (`self.LastHitActor`)))
      (bind _damagesphereradius (`/Game/CombatSystem/Weapons/Grenade/BP_Grenade.DamageSphereRadius` _granadeblueprint))
      (`GameplayStatics.ApplyDamage` _hitactor (`KismetMathLibrary.FClamp` (- (`self.MaxGrenadeDamage`) (* (/ (`KismetMathLibrary.FClamp` (`KismetMathLibrary.VSize` (- (`Actor.K2_GetActorLocation` _granadeblueprint) (`Actor.K2_GetActorLocation` _hitactor))) 0.0 _damagesphereradius) _damagesphereradius) (`self.DistanceMultiplier`))) (`self.MinGrenadeDamage`) (`self.MaxGrenadeDamage`)))
      (set `self.LastHitActor` _hitactor)))
  (`self.K2_EndAbility`))

(event `self.K2_OnEndAbility`
  (params (bWasCancelled :type Boolean))
  (set `self.LastHitActor` null))