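; Gameplay ability that applies incoming damage to a character and handles its hit reaction or death.
; It stops the active montage, then subtracts taken damage from health through character interface messages.
; Survivors play a front or back hit montage chosen by world yaw toward the hit location.
; At zero health it adds a dead tag, ragdolls, then after a delay destroys weapons and actor and hides the HUD.
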(event `self.K2_ActivateAbility`
  (bind _returnvalue (`self.GetAvatarActorFromActorInfo`))
  (bind _returnvalue_2 (`SkeletalMeshComponent.GetAnimInstance` (`Actor.GetComponentByClass` (`self.GetAvatarActorFromActorInfo`) "/Script/Engine.SkeletalMeshComponent")))
  (`self.K2_CommitAbility`)
  (`AnimInstance.Montage_Stop` _returnvalue_2 0.0 (`AnimInstance.GetCurrentActiveMontage` _returnvalue_2))
  (bind (_currenthealth _maxhealth _takendamage) (message `/Game/CombatSystem/Interfaces/BPI_BaseCharacter.GetCharacterHealth` _returnvalue))
  (bind _returnvalue_3 (`KismetMathLibrary.FClamp` (- _currenthealth _takendamage) 0.0 _maxhealth))
  (message `/Game/CombatSystem/Interfaces/BPI_BaseCharacter.SetCurrentHealth` _returnvalue _returnvalue_3)
  (if (<= _returnvalue_3 0.0)
    (`self.CharacterDeath`)
    (else
      (`self.PlayHitReactionMontage`))))

(event `PlayHitReactionMontage`
  (bind _returnvalue (`self.GetAvatarActorFromActorInfo`))
  (bind _hitlocation (message `/Game/CombatSystem/Interfaces/BPI_BaseCharacter.GetHitLocation` _returnvalue))
  (bind (_returnvalue_roll _returnvalue_pitch _returnvalue_yaw) (`KismetMathLibrary.BreakRotator` (`KismetMathLibrary.FindLookAtRotation` (`Actor.K2_GetActorLocation` _returnvalue) _hitlocation)))
  (`AbilityTask_PlayMontageAndWait.CreatePlayMontageAndWaitProxy` "None" (select `bool` (`KismetMathLibrary.InRange_FloatFloat` _returnvalue_yaw (`self.MinBackAngle`) (`self.MaxBackAngle`)) :`false` "/Game/CombatSystem/Animations/MM_HitReact_Back_Med_01_Montage.MM_HitReact_Back_Med_01_Montage" :`true` "/Game/CombatSystem/Animations/MM_HitReact_Front_Med_01_Montage.MM_HitReact_Front_Med_01_Montage" :!type "AnimMontage Object Reference")
    (:`OnCompleted`
      _)
    (:`OnInterrupted`
      _))
  (`self.K2_EndAbility`))

(event `CharacterDeath`
  (bind _returnvalue (`self.GetAvatarActorFromActorInfo`))
  (bind _returnvalue_2 (`self.GetAvatarActorFromActorInfo`))
  (bind _returnvalue_3 (`Actor.GetComponentByClass` _returnvalue "/Script/Engine.SkeletalMeshComponent"))
  (`AbilitySystemBlueprintLibrary.AddLooseGameplayTags` _returnvalue (`BlueprintGameplayTagLibrary.MakeLiteralGameplayTagContainer` (struct :`GameplayTags` (struct :`(TagName` "Character.States.IsDead")))))
  (`PrimitiveComponent.SetSimulatePhysics` _returnvalue_3 true)
  (`SkeletalMeshComponent.SetPhysicsBlendWeight` _returnvalue_3 (`self.DefaultPhysicsBlendWeightValue`))
  (`PrimitiveComponent.SetCollisionEnabled` _returnvalue_3 "QueryAndPhysics")
  (`KismetSystemLibrary.Delay` (`self.DestroyActorDelayTime`))
  (if (`KismetSystemLibrary.DoesImplementInterface` _returnvalue_2 "/Game/CombatSystem/Interfaces/BPI_BaseCharacter.BPI_BaseCharacter_C")
    (bind (_mainweapon _secondweapon) (message `/Game/CombatSystem/Interfaces/BPI_BaseCharacter.GetCharacterWeapons` _returnvalue_2))
    (for _array_element (`|MakeArray` _mainweapon _secondweapon)
      (`/Engine/EditorBlueprintResources/StandardMacros.IsValid` _array_element
        (:`Is Valid`
          (`Actor.K2_DestroyActor` _array_element))))
    (bind _charcaterhud (message `/Game/CombatSystem/Interfaces/BPI_BaseCharacter.GetCharacterHud` _returnvalue_2))
    (`/Engine/EditorBlueprintResources/StandardMacros.IsValid` _charcaterhud
      (:`Is Valid`
        (`Widget.SetVisibility` _charcaterhud "Hidden"))
      (:`Is Not Valid`
        _))
    (`Actor.K2_DestroyActor` (`self.GetAvatarActorFromActorInfo`))
    (`self.K2_EndAbility`)))