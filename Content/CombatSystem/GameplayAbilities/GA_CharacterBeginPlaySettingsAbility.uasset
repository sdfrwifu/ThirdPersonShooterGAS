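; Gameplay ability that initializes a character: weapons, anim instance, hidden HUD, and starting effects and abilities.
; SpawnWeapons finds the DT_CharacterClassStats row by the avatar's class name, spawns and attaches the main and optional second weapon, and applies GE_IsMainWeapon.
; It also caches the avatar and ability system component used by later steps.
; Weapon and anim instance references reach the character through BPI_CharacterVariablesSet; effects and abilities come from arrays.
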(event `self.K2_ActivateAbility`
  (`self.SpawnWeapons`)
  (`self.SetCharacterAnimInstance`)
  (`self.AddCharacterHud`)
  (`self.ApplyGameplayEffects`)
  (`self.GiveGameplayAbilities`))

(fn `AddCharacterHud`
  (bind _returnvalue (`|GenericCreateObject` "/Game/CombatSystem/Hud/CharacterHud.CharacterHud_C"))
  (bind _output_get (set `/Game/CombatSystem/Components/BP_CharacterComponent.CharacterHUD` _returnvalue (`Actor.GetComponentByClass` (`self.AvatarActor`) "/Game/CombatSystem/Components/BP_CharacterComponent.BP_CharacterComponent_C")))
  (`UserWidget.AddToViewport` _output_get 0)
  (`Widget.SetVisibility` _output_get "Hidden"))

(fn `ApplyGameplayEffects`
  (locals (EffectsArray :type "Array of GameplayEffect Class Reference"))
  (for _array_element (`local.EffectsArray`)
    (`AbilitySystemComponent.BP_ApplyGameplayEffectToSelf` :`self` (`self.AbilitySystemComponent`) :`GameplayEffectClass` _array_element)))

(fn `GiveGameplayAbilities`
  (locals (AbilitiesArray :type "Array of GameplayAbility Class Reference"))
  (for _array_element (`local.AbilitiesArray`)
    (`AbilitySystemComponent.K2_GiveAbility` (`self.AbilitySystemComponent`) _array_element 0 -1)))

(fn `SetCharacterAnimInstance`
  (bind _avataractor (`self.AvatarActor`))
  (if (`KismetSystemLibrary.DoesImplementInterface` _avataractor "/Game/CombatSystem/Interfaces/BPI_CharacterVariablesSet.BPI_CharacterVariablesSet_C")
    (message `/Game/CombatSystem/Interfaces/BPI_CharacterVariablesSet.SetAnimInstance` _avataractor (`SkeletalMeshComponent.GetAnimInstance` (`Actor.GetComponentByClass` _avataractor "/Script/Engine.SkeletalMeshComponent")))))

(fn `SetShootingComponent`
  (params (CurrentWeapon :type "/Game/CombatSystem/Weapons/BP_BaseWeapon Object Reference"))
  (set `self.ShootingComponent` (`/Game/CombatSystem/Weapons/BP_BaseWeapon.ShootingComponent` CurrentWeapon)))

(fn `SpawnWeapons`
  (locals (LocalSecondWeapon :type "/Game/CombatSystem/Weapons/BP_BaseWeapon Object Reference") (LocalMainWeapon :type "/Game/CombatSystem/Weapons/BP_BaseWeapon Object Reference"))
  (bind _returnvalue (`self.GetAvatarActorFromActorInfo`))
  (bind _returnvalue_2 (`self.GetAvatarActorFromActorInfo`))
  (bind _avataractor (`self.AvatarActor`))
  (bind _localmainweapon (`local.LocalMainWeapon`))
  (bind _spawnweapontransform (`self.SpawnWeaponTransform`))
  (set `self.AvatarActor` _returnvalue_2)
  (set `self.AbilitySystemComponent` (`Actor.GetComponentByClass` _returnvalue_2 "/Script/GameplayAbilities.AbilitySystemComponent"))
  (bind _returnvalue_3 (`|GetDataTableRow` "/Game/CombatSystem/DataTables/DT_CharacterClassStats.DT_CharacterClassStats" (`KismetStringLibrary.Conv_StringToName` (`KismetSystemLibrary.GetClassDisplayName` (`GameplayStatics.GetObjectClass` _returnvalue_2))))
    (:`then`
      (`|ExecutionSequence`
        (:`then_0`
          (bind (_characterclass _health _mainweapon _secondweapon) (break `/Game/CombatSystem/Structures/S_CharacterClassStats_New` _returnvalue_3))
          (bind _returnvalue_4 (`|SpawnActorFromClass` (`.WeaponClass_15_2EE0215A41C4F8CE701A2992F4D228EF` (break `/Game/CombatSystem/Structures/S_WeaponClassStats` _mainweapon)) _spawnweapontransform "AlwaysSpawn" "MultiplyWithRoot" _avataractor null))
          (bind _output_get (set `local.LocalMainWeapon` _returnvalue_4))
          (`self.SetShootingComponent` _output_get)
          (`/Game/CombatSystem/Components/BP_BaseShootingComponent.AttachWeapon` (`Actor.GetComponentByClass` _localmainweapon "/Game/CombatSystem/Components/BP_BaseShootingComponent.BP_BaseShootingComponent_C") _localmainweapon)
          (`AbilitySystemComponent.BP_ApplyGameplayEffectToSelf` :`self` (`self.AbilitySystemComponent`) :`GameplayEffectClass` "/Game/CombatSystem/GameplayAbilities/CharacterStates/GE_IsMainWeapon.GE_IsMainWeapon_C")
          (if (`KismetSystemLibrary.DoesImplementInterface` _returnvalue "/Game/CombatSystem/Interfaces/BPI_CharacterVariablesSet.BPI_CharacterVariablesSet_C") :!label _label
            (message `/Game/CombatSystem/Interfaces/BPI_CharacterVariablesSet.SetWeapons` _returnvalue (`local.LocalMainWeapon`) (`local.LocalSecondWeapon`))))
        (:`then_1`
          (bind _weaponclass (break `/Game/CombatSystem/Structures/S_WeaponClassStats` _secondweapon))
          (if (`KismetSystemLibrary.IsValidClass` _weaponclass)
            (bind _returnvalue_5 (`|SpawnActorFromClass` _weaponclass _spawnweapontransform "AlwaysSpawn" "MultiplyWithRoot" _avataractor null))
            (bind _output_get_2 (set `local.LocalSecondWeapon` _returnvalue_5))
            (`/Game/CombatSystem/Components/BP_BaseShootingComponent.AttachSecondWeapon` (`Actor.GetComponentByClass` _output_get_2 "/Game/CombatSystem/Components/BP_BaseShootingComponent.BP_BaseShootingComponent_C") _output_get_2)
            (goto _label)))))))