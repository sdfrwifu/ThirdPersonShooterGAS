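; BP_BaseWeapon is a base weapon that holds ammo, clip size, damage and fire rate, and exposes them through GetWeaponStats.
; SetAmmo refills the clip and writes the count to the HUD widget obtained from its owner, while SetCurrentAmmo only stores a supplied count.
; SpawnSoundAndFX plays the fire emitter and sound at the Muzzle.
; It contains no firing or damage logic.
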(event `self.ReceiveBeginPlay`)

(event `/Game/CombatSystem/Interfaces/BPI_Weapon.SetCurrentAmmo`
  (params (CurrentAmmo :type "Float (double-precision)"))
  (set `self.CurrentAmountOfAmmo` CurrentAmmo))

(fn `GetWeaponStats`
  (returns (CurrentAmmo :type "Float (double-precision)") (ClipAmount :type "Float (double-precision)") (WeaponDamage :type "Float (double-precision)") (WeaponFireRate :type "Float (double-precision)"))
  (return (`self.CurrentAmountOfAmmo`) (`self.ClipAmount`) (`self.WeaponDamage`) (`self.WeaponFireRate`)))

(fn `SetAmmo`
  (set `self.CurrentAmountOfAmmo` (`self.ClipAmount`))
  (bind _charcaterhud (message `/Game/CombatSystem/Interfaces/BPI_BaseCharacter.GetCharacterHud` (`self.GetOwner`)))
  (`/Engine/EditorBlueprintResources/StandardMacros.IsValid` _charcaterhud
    (:`Is Valid`
      (`TextBlock.SetText` (`/Game/CombatSystem/Hud/CharacterHud.AmmoAmount` _charcaterhud) (`KismetTextLibrary.Conv_DoubleToText` (`self.CurrentAmountOfAmmo`) "HalfToEven")))))

(fn `SpawnSoundAndFX`
  (bind _muzzle (`self.Muzzle`))
  (bind _returnvalue (`SceneComponent.K2_GetComponentLocation` _muzzle))
  ;[0.006141 1 0] Comment
  (`GameplayStatics.SpawnEmitterAtLocation` (`self.FireEmitter`) _returnvalue (`SceneComponent.K2_GetComponentRotation` _muzzle))
  (`GameplayStatics.SpawnSoundAtLocation` (`self.FireSound`) _returnvalue (struct) 1.0 1.0 0.0 null null))

(fn `UserConstructionScript`)