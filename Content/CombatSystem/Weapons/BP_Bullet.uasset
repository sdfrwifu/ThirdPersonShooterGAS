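; BP_Bullet is a projectile that damages third-person characters it overlaps, other than its owner, then destroys itself.
; The construction script sets the projectile movement's initial and maximum speed from its variables.
; On a valid hit it applies damage and plays a hit reaction montage at the bullet's location.
; Damage comes from the hit character's own class data, not the shooter's, choosing main or second weapon by that character's gameplay tag.
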(event `self.ReceiveBeginPlay`)

(event `self.DamageCollision.OnComponentBeginOverlap`
  (params (OverlappedComponent :type "PrimitiveComponent Object Reference") (OtherActor :type "Actor Object Reference") (OtherComp :type "PrimitiveComponent Object Reference") (OtherBodyIndex :type Integer) (bFromSweep :type Boolean) (SweepResult :type "HitResult Structure (by ref)"))
  (bind _asbp_base_third_person_character (cast `/Game/CombatSystem/Characters/BP_BaseThirdPersonCharacter` OtherActor))
  (if (!= OtherActor (`self.GetOwner`))
    (bind (_characterclass _health _mainweapon _secondweapon) (`/Game/CombatSystem/Components/BP_BaseShootingComponent.GetCharacterClassDataInfo` (`/Game/CombatSystem/Characters/BP_BaseThirdPersonCharacter.ShootingComponent` _asbp_base_third_person_character)))
    (`GameplayStatics.ApplyDamage` _asbp_base_third_person_character (`KismetMathLibrary.SelectFloat` (`.Damage_8_B282817843B7956B706AB79119A1B644` (break `/Game/CombatSystem/Structures/S_WeaponClassStats` _mainweapon)) (`.Damage_8_B282817843B7956B706AB79119A1B644` (break `/Game/CombatSystem/Structures/S_WeaponClassStats` _secondweapon)) (`GameplayTagAssetInterface.HasMatchingGameplayTag` (`/Game/CombatSystem/Characters/BP_BaseThirdPersonCharacter.MyAbilitySystemComponent` _asbp_base_third_person_character) (struct :`TagName` "WeaponState.IsMainWeapon"))))
    (`/Game/CombatSystem/Components/BP_CharacterComponent.PlayHitReactionMontage` (`/Game/CombatSystem/Characters/BP_BaseThirdPersonCharacter.CharacterComponent` _asbp_base_third_person_character) _asbp_base_third_person_character (`self.K2_GetActorLocation`))
    (`self.K2_DestroyActor`)))

(fn `UserConstructionScript`
  (bind _projectilemovement (`self.ProjectileMovement`))
  (set `ProjectileMovementComponent.InitialSpeed` (`self.DefaultSpeed`) _projectilemovement)
  (set `ProjectileMovementComponent.MaxSpeed` (`self.MaxSpeed`) _projectilemovement))