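; Actor component that implements the sniper character's three abilities and its aiming and scoping behavior.
; The first applies timed damage ticks to a target; the second swaps weapons with a camera lerp and equip montage.
; The movement ability launches the character into temporary flight, with Tick switching fly speed by aiming tag.
; It binds to ShootingComponent events and uses Delay-reset flags for first and movement ability cooldowns.
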(event `self.ReceiveBeginPlay`
  (bind _asbp_sniper_third_person_character (cast `/Game/CombatSystem/Characters/BP_SniperThirdPersonCharacter` (`self.GetOwner`)))
  (set `self.BP_SniperThird PersonCharacter` _asbp_sniper_third_person_character)
  (`KismetSystemLibrary.DelayUntilNextTick`)
  (`self.BindEvents`))

(event `SniperAbilityDamageEvent`
  ;[0.006141 1 0] First Ability
  (`self.SniperAbilityDamage` (stale `SniperFirstAbility` DamagedActor)))

(event `SniperFirstAbility`
  (params (DamagedActor :type "Actor Object Reference"))
  ;[0.006141 1 0] First Ability
  (if (`self.IsAbilityActive`)
    (set `self.IsAbilityActive` false)
    (bind _returnvalue (`KismetSystemLibrary.K2_SetTimerDelegate` (delegate `SniperAbilityDamageEvent`) (`self.SniperAbilityTickTimeRate`) true))
    (set `self.SniperAbilityTimer` _returnvalue)
    (set `self.DoesSniperAbilityCooldownEnd` false)
    (`KismetSystemLibrary.Delay` 20.0)
    (set `self.DoesSniperAbilityCooldownEnd` true)))

(event `SniperSecondAbility`
  (params (SpawnedWeapon :type "Actor Object Reference"))
  (bind _bp_sniperthird_personcharacter (`self.BP_SniperThird PersonCharacter`))
  (bind _bp_sniperthird_personcharacter_2 (`self.BP_SniperThird PersonCharacter`))
  (bind _bp_sniperthird_personcharacter_3 (`self.BP_SniperThird PersonCharacter`))
  (bind _abp_manny (`/Game/CombatSystem/Characters/BP_BaseThirdPersonCharacter.ABP_Manny` _bp_sniperthird_personcharacter_2))
  (bind _shootingcomponent (`/Game/CombatSystem/Characters/BP_BaseThirdPersonCharacter.ShootingComponent` (`self.BP_SniperThird PersonCharacter`)))
  ;[0.006141 1 0] Sniper Swap Weapon / Second Ability
  (`CameraComponent.SetFieldOfView` (`/Game/CombatSystem/Characters/BP_BaseThirdPersonCharacter.ThirdPersonCamera` _bp_sniperthird_personcharacter) (`/Game/CombatSystem/Characters/BP_BaseThirdPersonCharacter.DefaultFOV` _bp_sniperthird_personcharacter))
  (set `/Game/CombatSystem/Components/BP_BaseShootingComponent.CanAim` false (`/Game/CombatSystem/Characters/BP_BaseThirdPersonCharacter.ShootingComponent` _bp_sniperthird_personcharacter))
  (set `self.CurrentSpringArmOffset` (`SpringArmComponent.SocketOffset` (`/Game/CombatSystem/Characters/BP_BaseThirdPersonCharacter.CameraBoom` (`self.BP_SniperThird PersonCharacter`))))
  (bind _returnvalue (`KismetSystemLibrary.K2_SetTimerDelegate` (delegate `ReturnCamera`) (`self.AimingLerpTickTimeRate`) true))
  (set `self.ReturnCameraTimer` _returnvalue)
  (`/Game/CombatSystem/Components/BP_BaseShootingComponent.NotAimingSettings` _shootingcomponent)
  (`/Game/CombatSystem/Components/BP_BaseShootingComponent.AttachWeapon` _shootingcomponent SpawnedWeapon)
  (`/Game/CombatSystem/Components/BP_BaseShootingComponent.SetAmmo` _shootingcomponent)
  (`self.BindEvents`)
  (`self.SetNotAimingSettings`)
  (set `CharacterMovementComponent.MaxWalkSpeed` (`/Game/CombatSystem/Components/BP_BaseShootingComponent.CurrentMaxCharacterSpeed` (`/Game/CombatSystem/Characters/BP_BaseThirdPersonCharacter.ShootingComponent` _bp_sniperthird_personcharacter_3)) (`Character.CharacterMovement` _bp_sniperthird_personcharacter_3))
  (set `/Game/Characters/Mannequins/Animations/ABP_Manny.IsUpperBody` true _abp_manny)
  (`|PlayMontage` (`Character.Mesh` _bp_sniperthird_personcharacter_2) "/Game/CombatSystem/Animations/AM_MM_Rifle_Equip.AM_MM_Rifle_Equip"
    (:`OnBlendOut`
      (set `/Game/Characters/Mannequins/Animations/ABP_Manny.IsUpperBody` false _abp_manny)
      (set `/Game/CombatSystem/Components/BP_BaseShootingComponent.CanAim` true (`/Game/CombatSystem/Characters/BP_BaseThirdPersonCharacter.ShootingComponent` _bp_sniperthird_personcharacter_2)))))

(event `ReturnCamera`
  ;[0.006141 1 0] Sniper Swap Weapon / Second Ability
  (`self.ReturnCameraChange`))

(event `LaunchCharacterUp`
  (bind _bp_sniperthird_personcharacter (`self.BP_SniperThird PersonCharacter`))
  (bind _charactermovement (`Character.CharacterMovement` _bp_sniperthird_personcharacter))
  ;[0.006141 1 0] Sniper Movement Ability
  (`|ExecutionSequence`
    (:`then_0`
      (set `self.DoesSniperMovementAbilityCooldownEnd` false)
      (`KismetSystemLibrary.Delay` 20.0)
      (set `self.DoesSniperMovementAbilityCooldownEnd` true))
    (:`then_1`
      (`Character.LaunchCharacter` _bp_sniperthird_personcharacter (0.0 0.0 1500.0) false false)
      (`CharacterMovementComponent.SetMovementMode` _charactermovement "MOVE_Flying" 0)
      (set `self.IsFlying` true)
      (`KismetSystemLibrary.Delay` 10.0)
      (set `self.IsFlying` false)
      (`CharacterMovementComponent.SetMovementMode` _charactermovement "MOVE_Falling" 0))))

(event `FlyUpDown`
  (params (ScaleValue :type "Float (double-precision)"))
  (bind _bp_sniperthird_personcharacter (`self.BP_SniperThird PersonCharacter`))
  ;[0.006141 1 0] Sniper Movement Ability
  (if (`NavMovementComponent.IsFlying` (`Character.CharacterMovement` _bp_sniperthird_personcharacter))
    (`Pawn.AddMovementInput` _bp_sniperthird_personcharacter (`Actor.GetActorUpVector` (`Pawn.GetController` _bp_sniperthird_personcharacter)) ScaleValue false)))

(event `self.ReceiveTick`
  (params (DeltaSeconds :type "Float (single-precision)"))
  (bind _bp_sniperthird_personcharacter (`self.BP_SniperThird PersonCharacter`))
  (bind _charactermovement (`Character.CharacterMovement` _bp_sniperthird_personcharacter))
  ;[0.006141 1 0] Flying Mode
  (if (`self.IsFlying`)
    (`CharacterMovementComponent.SetMovementMode` _charactermovement "MOVE_Flying" 0)
    (if (`GameplayTagAssetInterface.HasMatchingGameplayTag` (`/Game/CombatSystem/Characters/BP_BaseThirdPersonCharacter.AbilitySystemComponent` _bp_sniperthird_personcharacter) (struct :`TagName` "PlayerState.IsAiming"))
      (set `CharacterMovementComponent.MaxFlySpeed` (`self.MaxAimingFlyingSpeed`) _charactermovement)
      (else
        (set `CharacterMovementComponent.MaxFlySpeed` (`self.MaxDefaultFlyingSpeed`) _charactermovement)))))

(fn `BindEvents`
  (bind _shootingcomponent (`/Game/CombatSystem/Characters/BP_BaseThirdPersonCharacter.ShootingComponent` (`self.BP_SniperThird PersonCharacter`)))
  (add `/Game/CombatSystem/Components/BP_BaseShootingComponent.OnHeadHit` _shootingcomponent (`|CreateDelegate` :!event `SetHeadDamageMultiplier`))
  (add `/Game/CombatSystem/Components/BP_BaseShootingComponent.OnFirstSniperAbility` _shootingcomponent (`|CreateDelegate` :!event `SniperFirstAbility`))
  (add `/Game/CombatSystem/Components/BP_BaseShootingComponent.OnNotAimingSettings` _shootingcomponent (`|CreateDelegate` :!event `SetNotAimingSettings`))
  (add `/Game/CombatSystem/Components/BP_BaseShootingComponent.OnAimingSetFOV` _shootingcomponent (`|CreateDelegate` :!event `SetAimingFOV`)))

(fn `ReturnCameraChange`
  (locals (LocalSpringArmChangeRate :type "Float (double-precision)" :default 0.025) (LocalDefaultSpringArmOffset :type "Vector Structure") (LocalLerpEndAlpha :type "Float (double-precision)" :default 1.0))
  (bind _output_get (set `self.SpringArmAlpha` (+ (`self.SpringArmAlpha`) (`local.LocalSpringArmChangeRate`))))
  (set `SpringArmComponent.SocketOffset` (`KismetMathLibrary.VLerp` (`self.CurrentSpringArmOffset`) (`local.LocalDefaultSpringArmOffset`) _output_get) (`/Game/CombatSystem/Characters/BP_BaseThirdPersonCharacter.CameraBoom` (`self.BP_SniperThird PersonCharacter`)))
  (if (>= (`self.SpringArmAlpha`) (`local.LocalLerpEndAlpha`))
    (`KismetSystemLibrary.K2_ClearAndInvalidateTimerHandle` (`self.ReturnCameraTimer`))))

(fn `SetAimingFOV`
  (locals (LocalScopingFOV :type "Float (single-precision)" :default 27.0))
  (bind _bp_sniperthird_personcharacter (`self.BP_SniperThird PersonCharacter`))
  (bind _characterhud (`/Game/CombatSystem/Characters/BP_BaseThirdPersonCharacter.CharacterHud` _bp_sniperthird_personcharacter))
  (bind _aimimage (`/Game/CombatSystem/Hud/CharacterHud.AimImage` _characterhud))
  (if (`GameplayTagAssetInterface.HasMatchingGameplayTag` (`/Game/CombatSystem/Characters/BP_BaseThirdPersonCharacter.AbilitySystemComponent` (`self.BP_SniperThird PersonCharacter`)) (struct :`TagName` "PlayerState.IsScoping"))
    (`CameraComponent.SetFieldOfView` (`/Game/CombatSystem/Characters/BP_BaseThirdPersonCharacter.ThirdPersonCamera` _bp_sniperthird_personcharacter) (`local.LocalScopingFOV`))
    (`Widget.SetVisibility` _aimimage "Hidden")
    (`Widget.SetVisibility` (`/Game/CombatSystem/Hud/CharacterHud.ScopeImage` _characterhud) "Visible")
    (else
      (`Widget.SetVisibility` (`/Game/CombatSystem/Hud/CharacterHud.ScopeImage` _characterhud) "Hidden")
      (`Widget.SetVisibility` _aimimage "Visible"))))

(fn `SetHeadDamageMultiplier`
  (locals (LocalHeadDamageMultiplier :type "Float (double-precision)" :default 1.5))
  (set `/Game/CombatSystem/Components/BP_BaseShootingComponent.DamageMultiplier` (`local.LocalHeadDamageMultiplier`) (`/Game/CombatSystem/Characters/BP_BaseThirdPersonCharacter.ShootingComponent` (`self.BP_SniperThird PersonCharacter`))))

(fn `SetNotAimingSettings`
  (bind _bp_sniperthird_personcharacter (`self.BP_SniperThird PersonCharacter`))
  (bind _bp_sniperthird_personcharacter_2 (`self.BP_SniperThird PersonCharacter`))
  (set `/Game/CombatSystem/Components/BP_BaseShootingComponent.CurrentMaxCharacterSpeed` (`KismetMathLibrary.SelectFloat` (`self.MaxPistolCharacterSpeed`) (`self.MaxDefaultCharacterSpeed`) (`/Game/CombatSystem/Characters/BP_SniperThirdPersonCharacter.IsCurrentWeaponPistol` _bp_sniperthird_personcharacter_2)) (`/Game/CombatSystem/Characters/BP_BaseThirdPersonCharacter.ShootingComponent` _bp_sniperthird_personcharacter_2))
  (if (`GameplayTagAssetInterface.HasMatchingGameplayTag` (`/Game/CombatSystem/Characters/BP_BaseThirdPersonCharacter.AbilitySystemComponent` _bp_sniperthird_personcharacter_2) (struct :`TagName` "PlayerState.IsScoping"))
    (`CameraComponent.SetFieldOfView` (`/Game/CombatSystem/Characters/BP_BaseThirdPersonCharacter.ThirdPersonCamera` _bp_sniperthird_personcharacter) (`/Game/CombatSystem/Characters/BP_BaseThirdPersonCharacter.DefaultFOV` _bp_sniperthird_personcharacter))))

(fn `SniperAbilityDamage`
  (params (DamagedActor :type "Actor Object Reference"))
  (locals (LocalSniperAbilityTickDamage :type "Float (double-precision)" :default 5.0) (LocalMaxAmountOfTicks :type Integer :default 4))
  (`GameplayStatics.ApplyDamage` DamagedActor (`local.LocalSniperAbilityTickDamage`))
  (bind _result (`/Engine/EditorBlueprintResources/StandardMacros.IncrementInt` (`self.AbilityAmountOfTicks`))
    (:`  `
      (if (== _result (`local.LocalMaxAmountOfTicks`))
        (set `self.AbilityAmountOfTicks` 0)
        (`KismetSystemLibrary.K2_ClearAndInvalidateTimerHandle` (`self.SniperAbilityTimer`))))))