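; Character component in the combat system that caches its third-person owner and plays hit reactions on struck characters.
; It picks a front or back montage from the world-space yaw between the hit actor's location and the hit point.
; It enables upper-body animation on the victim's ABP_Manny, clearing it on blend-out only if the owner's weapon, not the victim's, reports reload completed.
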(event `self.ReceiveBeginPlay`
  (bind _asbp_base_third_person_character (cast `/Game/CombatSystem/Characters/BP_BaseThirdPersonCharacter` (`self.GetOwner`)))
  (set `self.BaseThirdPersonCharacter` _asbp_base_third_person_character))

(event `PlayHitReactionMontage`
  (params (HitActor :type "Actor Object Reference") (HitLocation :type "Vector Structure"))
  (bind (_returnvalue_roll _returnvalue_pitch _returnvalue_yaw) (`KismetMathLibrary.BreakRotator` (`KismetMathLibrary.FindLookAtRotation` (`Actor.K2_GetActorLocation` HitActor) HitLocation)))
  ;[0.006141 1 0] Hit Reaction
  (bind _asbp_base_third_person_character (cast `/Game/CombatSystem/Characters/BP_BaseThirdPersonCharacter` HitActor))
  (bind _asabp_manny (cast `/Game/Characters/Mannequins/Animations/ABP_Manny` (`SkeletalMeshComponent.GetAnimInstance` (`Character.Mesh` _asbp_base_third_person_character)) :!pure true))
  (set `/Game/Characters/Mannequins/Animations/ABP_Manny.IsUpperBody` true _asabp_manny)
  (if (`KismetMathLibrary.InRange_FloatFloat` _returnvalue_yaw -90.0 90.0)
    (`|PlayMontage` (`Character.Mesh` _asbp_base_third_person_character) "/Game/CombatSystem/Animations/MM_HitReact_Front_Med_01_Montage.MM_HitReact_Front_Med_01_Montage"
      (:`OnBlendOut`
        _))
    (else
      (`|PlayMontage` (`Character.Mesh` _asbp_base_third_person_character) "/Game/CombatSystem/Animations/MM_HitReact_Back_Med_01_Montage.MM_HitReact_Back_Med_01_Montage"
        (:`OnBlendOut`
          _))))
  ;;[1 1 1] doubtfull
  (if (`/Game/CombatSystem/Components/BP_BaseShootingComponent.IsReloadCompleted` (`/Game/CombatSystem/Weapons/BP_BaseWeapon.ShootingComponent` (`/Game/CombatSystem/Characters/BP_BaseThirdPersonCharacter.CurrentWeaponBlueprint` (`self.BaseThirdPersonCharacter`))))
    (set `/Game/Characters/Mannequins/Animations/ABP_Manny.IsUpperBody` false _asabp_manny)))